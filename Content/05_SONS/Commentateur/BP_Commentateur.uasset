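; Commentator actor that plays one random voice line from a single long Commentator sound, then destroys itself.
; On BeginPlay it picks a random segment index and starts a 2D sound at that segment's hard-coded start time.
; It waits for the gap to the next start time, then stops the sound, so one audio file serves as a bank of clips.
; Debug prints show its name and the clip length.
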(event EventBeginPlay
  (Variables|Default|SetNewVar (Math|Random|RandomIntegerinRange 0 25))
  (Development|PrintString "COMMENTATEUR" true true "(R=1.000000,G=0.000000,B=0.612064,A=1.000000)" 5.0)
  (bind _returnvalue (Audio|SpawnSound2D "/Game/05_SONS/Commentateur/Commentator.Commentator" 0.9 1.0 (Utilities|Select :Index (Variables|Default|GetNewVar) :Option%200 0.0 :Option%201 4.0 :Option%202 8.0 :Option%203 12.0 :Option%204 16.0 :Option%205 22.0 :Option%206 26.0 :Option%207 32.0 :Option%208 35.0 :Option%209 41.0 :Option%2010 46.0 :Option%2011 52.0 :Option%2012 6e+01 :Option%2013 66.0 :Option%2014 7e+01 :Option%2015 73.0 :Option%2016 76.0 :Option%2017 81.0 :Option%2018 85.0 :Option%2019 9e+01 :Option%2020 93.0 :Option%2021 97.0 :Option%2022 104.0 :Option%2023 111.0 :Option%2024 116.0 :Option%2025 123.0 :Option%2026 128.0) 0))
  (Development|PrintString (Utilities|String|ToString(Float) (- (Utilities|Select :Index (+ (Variables|Default|GetNewVar) 1) :Option%200 0.0 :Option%201 4.0 :Option%202 8.0 :Option%203 12.0 :Option%204 16.0 :Option%205 22.0 :Option%206 26.0 :Option%207 32.0 :Option%208 35.0 :Option%209 41.0 :Option%2010 46.0 :Option%2011 52.0 :Option%2012 6e+01 :Option%2013 66.0 :Option%2014 7e+01 :Option%2015 73.0 :Option%2016 76.0 :Option%2017 81.0 :Option%2018 85.0 :Option%2019 9e+01 :Option%2020 93.0 :Option%2021 97.0 :Option%2022 104.0 :Option%2023 111.0 :Option%2024 116.0 :Option%2025 123.0 :Option%2026 128.0) (Utilities|Select :Index (Variables|Default|GetNewVar) :Option%200 0.0 :Option%201 4.0 :Option%202 8.0 :Option%203 12.0 :Option%204 16.0 :Option%205 22.0 :Option%206 26.0 :Option%207 32.0 :Option%208 35.0 :Option%209 41.0 :Option%2010 46.0 :Option%2011 52.0 :Option%2012 6e+01 :Option%2013 66.0 :Option%2014 7e+01 :Option%2015 73.0 :Option%2016 76.0 :Option%2017 81.0 :Option%2018 85.0 :Option%2019 9e+01 :Option%2020 93.0 :Option%2021 97.0 :Option%2022 104.0 :Option%2023 111.0 :Option%2024 116.0 :Option%2025 123.0 :Option%2026 128.0))))
  (Utilities|FlowControl|Delay (- (Utilities|Select :Index (+ (Variables|Default|GetNewVar) 1) :Option%200 0.0 :Option%201 4.0 :Option%202 8.0 :Option%203 12.0 :Option%204 16.0 :Option%205 22.0 :Option%206 26.0 :Option%207 32.0 :Option%208 35.0 :Option%209 41.0 :Option%2010 46.0 :Option%2011 52.0 :Option%2012 6e+01 :Option%2013 66.0 :Option%2014 7e+01 :Option%2015 73.0 :Option%2016 76.0 :Option%2017 81.0 :Option%2018 85.0 :Option%2019 9e+01 :Option%2020 93.0 :Option%2021 97.0 :Option%2022 104.0 :Option%2023 111.0 :Option%2024 116.0 :Option%2025 123.0 :Option%2026 128.0) (Utilities|Select :Index (Variables|Default|GetNewVar) :Option%200 0.0 :Option%201 4.0 :Option%202 8.0 :Option%203 12.0 :Option%204 16.0 :Option%205 22.0 :Option%206 26.0 :Option%207 32.0 :Option%208 35.0 :Option%209 41.0 :Option%2010 46.0 :Option%2011 52.0 :Option%2012 6e+01 :Option%2013 66.0 :Option%2014 7e+01 :Option%2015 73.0 :Option%2016 76.0 :Option%2017 81.0 :Option%2018 85.0 :Option%2019 9e+01 :Option%2020 93.0 :Option%2021 97.0 :Option%2022 104.0 :Option%2023 111.0 :Option%2024 116.0 :Option%2025 123.0 :Option%2026 128.0)))
  (Audio|Components|Audio|Stop _returnvalue)
  (Actor|DestroyActor))

(fn ConstructionScript)