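; BP_WallBlock is a wall block that reports player hits to BP_FirstPersonGameMode when its Box component is overlapped.
; BeginPlay caches the game mode and both players via GetActorOfClass, with no class set for P1, and sets both player flags true.
; Overlap branches call Player1Hit or Player2Hit with debug prints, but never compare against the cached players, so the Player 1 branch takes priority.
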(event OnComponentBeginOverlap(Box)
  (params (OverlappedComponent :type Primitive%20Component%20Object%20Reference) (OtherActor :type Actor%20Object%20Reference) (OtherComp :type Primitive%20Component%20Object%20Reference) (OtherBodyIndex :type Integer) (bFromSweep :type Boolean) (SweepResult :type Hit%20Result%20Structure%20%28by%20ref%29))
  (bind _gamemode (Variables|Default|GetGameMode))
  (Development|PrintString "Hello")
  (if (and (Collision|IsOverlappingActor OverlappedComponent OtherActor :!class /Script/Engine.PrimitiveComponent) (Variables|Default|GetP1Bool))
    (Default|Player1Hit _gamemode)
    (Development|PrintString "Hello 22")
    (elif (and (Collision|IsOverlappingActor OverlappedComponent OtherActor :!class /Script/Engine.PrimitiveComponent) (Variables|Default|GetP2Bool))
      (Default|Player2Hit _gamemode)
      (Development|PrintString "Hello 33")
      (else
        (Development|PrintString "Hello 44")))))

(event EventBeginPlay
  (bind _returnvalue (Actor|GetActorOfClass "/Game/01_Character/Blueprints/BP_FirstPersonGameMode.BP_FirstPersonGameMode_C"))
  (Variables|Default|SetGameMode _returnvalue)
  (bind _returnvalue_2 (Actor|GetActorOfClass 0))
  (Variables|Default|SetP1 _returnvalue_2)
  (Variables|Default|SetP1Bool true)
  (bind _returnvalue_3 (Actor|GetActorOfClass "/Game/01_Character/Blueprints/BP_CharacterP2.BP_CharacterP2_C"))
  (Variables|Default|SetP2 _returnvalue_3)
  (Variables|Default|SetP2Bool true))

(fn ConstructionScript)