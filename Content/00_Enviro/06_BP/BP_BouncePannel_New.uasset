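; Environment panel Blueprint that animates texture offsets on its Screen component through a dynamic material instance.
; BeginPlay creates instances for two material slots, but the second overwrites DMDecal, so only the Master_Screen_Inst slot animates.
; Random branches pick one of four delayed motion variants to desynchronize panels.
; Each variant chains an X-offset and a Y-offset timeline through FlipFlops, alternating axes and directions in an endless loop.
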(event EventBeginPlay
  (bind _screen (Variables|Default|GetScreen))
  (Utilities|FlowControl|Sequence
    (:then_0
      (bind _returnvalue (Rendering|Material|CreateDynamicMaterialInstance _screen 0 0 "None" :!class /Script/Engine.PrimitiveComponent))
      (bind _output_get (Variables|Default|SetDM_Decal _returnvalue))
      (Rendering|Material|SetMaterial _screen 0 _output_get))
    (:then_1
      ;[0.15 0.15 0.15 0.5 50] OLD
      (Utilities|FlowControl|Sequence
        (:then_0
          (bind _returnvalue_2 (Rendering|Material|CreateDynamicMaterialInstance (Variables|Default|GetScreen) 1 "/Game/03_VFX/02_Material/00_Master/Master_Screen_Inst.Master_Screen_Inst" "None" :!class /Script/Engine.PrimitiveComponent))
          (bind _output_get_2 (Variables|Default|SetDM_Decal _returnvalue_2))
          (Rendering|Material|SetMaterial (Variables|Default|GetScreen) 1 _output_get_2))
        (:then_1
          (if (Math|Random|RandomBool)
            (if (Math|Random|RandomBool)
              (Utilities|FlowControl|Delay (Math|Random|RandomFloatinRange 0.0 2.0))
              (Rendering|Material|SetScalarParameterValue (Variables|Default|GetDM_Decal) "T_Y_Offset" 0.5 :!class /Script/Engine.MaterialInstanceDynamic)
              (bind _t_offset (Timeline|Timeline_3 PlayFromStart)
                (:Update
                  (Rendering|Material|SetScalarParameterValue (Variables|Default|GetDM_Decal) "T_X_Offset" _t_offset :!class /Script/Engine.MaterialInstanceDynamic))
                (:Finished
                  (Utilities|FlowControl|FlipFlop
                    (:A
                      (bind _t_offset_2 (Timeline|Timeline_4 ReverseFromEnd)
                        (:Update
                          (Rendering|Material|SetScalarParameterValue (Variables|Default|GetDM_Decal) "T_Y_Offset" _t_offset_2 :!class /Script/Engine.MaterialInstanceDynamic))
                        (:Finished
                          (Utilities|FlowControl|FlipFlop
                            (:A
                              (Timeline|Timeline_3 ReverseFromEnd))
                            (:B
                              (Timeline|Timeline_3 PlayFromStart))))))
                    (:B
                      (Timeline|Timeline_4 PlayFromStart)))))
              (else
                (Utilities|FlowControl|Delay (Math|Random|RandomFloatinRange 0.0 5.0))
                (Rendering|Material|SetScalarParameterValue (Variables|Default|GetDM_Decal) "T_Y_Offset" 0.5 :!class /Script/Engine.MaterialInstanceDynamic)
                (bind _t_offset_3 (Timeline|Timeline_5 ReverseFromEnd)
                  (:Update
                    (Rendering|Material|SetScalarParameterValue (Variables|Default|GetDM_Decal) "T_X_Offset" _t_offset_3 :!class /Script/Engine.MaterialInstanceDynamic))
                  (:Finished
                    (Utilities|FlowControl|FlipFlop
                      (:A
                        (bind _t_offset_4 (Timeline|Timeline_6 ReverseFromEnd)
                          (:Update
                            (Rendering|Material|SetScalarParameterValue (Variables|Default|GetDM_Decal) "T_Y_Offset" _t_offset_4 :!class /Script/Engine.MaterialInstanceDynamic))
                          (:Finished
                            (Utilities|FlowControl|FlipFlop
                              (:A
                                (Timeline|Timeline_5 PlayFromStart))
                              (:B
                                (Timeline|Timeline_5 ReverseFromEnd))))))
                      (:B
                        (Timeline|Timeline_6 PlayFromStart)))))))
            (elif (Math|Random|RandomBool)
              (Utilities|FlowControl|Delay (Math|Random|RandomFloatinRange 0.0 2.0))
              (bind _t_offset_5 (Timeline|Timeline PlayFromStart)
                (:Update
                  (Rendering|Material|SetScalarParameterValue (Variables|Default|GetDM_Decal) "T_X_Offset" _t_offset_5 :!class /Script/Engine.MaterialInstanceDynamic))
                (:Finished
                  (Utilities|FlowControl|FlipFlop
                    (:A
                      (bind _t_offset_6 (Timeline|Timeline_0 PlayFromStart)
                        (:Update
                          (Rendering|Material|SetScalarParameterValue (Variables|Default|GetDM_Decal) "T_Y_Offset" _t_offset_6 :!class /Script/Engine.MaterialInstanceDynamic))
                        (:Finished
                          (Utilities|FlowControl|FlipFlop
                            (:A
                              (Timeline|Timeline ReverseFromEnd))
                            (:B
                              (Timeline|Timeline PlayFromStart))))))
                    (:B
                      (Timeline|Timeline_0 ReverseFromEnd)))))
              (else
                (Utilities|FlowControl|Delay (Math|Random|RandomFloatinRange 0.0 5.0))
                (Rendering|Material|SetScalarParameterValue (Variables|Default|GetDM_Decal) "T_X_Offset" 0.5 :!class /Script/Engine.MaterialInstanceDynamic)
                (bind _t_offset_7 (Timeline|Timeline_1 ReverseFromEnd)
                  (:Update
                    (Rendering|Material|SetScalarParameterValue (Variables|Default|GetDM_Decal) "T_X_Offset" _t_offset_7 :!class /Script/Engine.MaterialInstanceDynamic))
                  (:Finished
                    (Utilities|FlowControl|FlipFlop
                      (:A
                        (bind _t_offset_8 (Timeline|Timeline_2 PlayFromStart)
                          (:Update
                            (Rendering|Material|SetScalarParameterValue (Variables|Default|GetDM_Decal) "T_Y_Offset" _t_offset_8 :!class /Script/Engine.MaterialInstanceDynamic))
                          (:Finished
                            (Utilities|FlowControl|FlipFlop
                              (:A
                                (Timeline|Timeline_1 PlayFromStart))
                              (:B
                                (Timeline|Timeline_1 ReverseFromEnd))))))
                      (:B
                        (Timeline|Timeline_2 ReverseFromEnd)))))))))))))

(fn ConstructionScript)