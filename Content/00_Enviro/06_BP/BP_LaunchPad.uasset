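; BP_LaunchPad is a launch pad that flings overlapping BP_Character_Manager characters along its arrow's forward direction.
; On Collision overlap it briefly switches the character to Flying, zeroes velocity, then calls LaunchCharacter with both overrides, scaled by LaunchPadVelocity.
; It immediately restores Walking mode and activates the NSJumpPadActivate effect.
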(event OnComponentBeginOverlap(Collision)
  (params (OverlappedComponent :type Primitive%20Component%20Object%20Reference) (OtherActor :type Actor%20Object%20Reference) (OtherComp :type Primitive%20Component%20Object%20Reference) (OtherBodyIndex :type Integer) (bFromSweep :type Boolean) (SweepResult :type Hit%20Result%20Structure%20%28by%20ref%29))
  (Utilities|IsValid OtherActor
    (:Is%20Valid
      (bind _asbp_character_manager (Utilities|Casting|CastToBP_Character_Manager OtherActor))
      (Pawn|Components|CharacterMovement|SetMovementMode (Variables|/Script/Engine.Character|GetCharacterMovement _asbp_character_manager) "MOVE_Flying" 0)
      (Variables|/Script/Engine.MovementComponent|SetVelocity (Variables|/Script/Engine.Character|GetCharacterMovement _asbp_character_manager) "0, 0, 0")
      (Character|LaunchCharacter _asbp_character_manager (* (Variables|Default|GetLaunchPad_Velocity) (Math|Vector|GetForwardVector (Variables|Default|GetArrow))) true true)
      (Pawn|Components|CharacterMovement|SetMovementMode (Variables|/Script/Engine.Character|GetCharacterMovement _asbp_character_manager) "MOVE_Walking" 0)
      (Components|Activation|Activate (Variables|Default|GetNS_JumpPadActivate) true))))

(fn ConstructionScript)