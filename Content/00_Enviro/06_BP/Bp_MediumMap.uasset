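; Bp_MediumMap is an environment Blueprint that, as wired, only caches a reference to one of the two player characters.
; A DoOnce on Tick uses the PLAYER12 flag to pick BP_Character_P1 or BP_Character_P2 via GetActorOfClass.
; Unconnected leftover nodes would switch a light from red to blue after a delay and rotate toward the chosen player, but they never run.
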(event EventTick
  (params (DeltaSeconds :type Float%20%28single-precision%29))
  (Utilities|FlowControl|Sequence
    (:then_0
      (Utilities|FlowControl|DoOnce false
        (:Completed
          (if (Variables|Default|GetPLAYER%201/2)
            (bind _returnvalue (Actor|GetActorOfClass "/Game/01_Character/Blueprints/00_Character/BP_Character_P1.BP_Character_P1_C"))
            (Variables|Default|SetPlayer%201 _returnvalue)
            (else
              (bind _returnvalue_2 (Actor|GetActorOfClass "/Game/01_Character/Blueprints/00_Character/BP_Character_P2.BP_Character_P2_C"))
              (Variables|Default|SetPlayer%202 _returnvalue_2))))))))

(event EventBeginPlay)

(fn ConstructionScript)