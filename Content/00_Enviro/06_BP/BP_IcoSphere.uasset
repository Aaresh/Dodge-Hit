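; BP_IcoSphere is an environment actor whose surface animates its color and glow when hit.
; BeginPlay caches the game mode and both player characters after a short delay, then gives the Plane mesh a dynamic material.
; Hits on Plane1 play a timeline blending that material between cyan and pink-red while varying emissive strength.
; A DoOnce gate blocks retriggering until the timeline finishes.
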(event OnComponentHit(Plane1)
  (params (HitComponent :type Primitive%20Component%20Object%20Reference) (OtherActor :type Actor%20Object%20Reference) (OtherComp :type Primitive%20Component%20Object%20Reference) (NormalImpulse :type Vector :default "0, 0, 0") (Hit :type Hit%20Result%20Structure%20%28by%20ref%29))
  (bind _dm_wall (Variables|Default|GetDM_Wall))
  (Utilities|FlowControl|DoOnce false
    (:Completed
      (bind _color (Timeline|Color PlayFromStart)
        (:Update
          (Rendering|Material|SetVectorParameterValue _dm_wall "Color" (Math|Color|Lerp(LinearColor) "(R=0.000000,G=0.783538,B=1.000000,A=1.000000)" "(R=1.000000,G=0.000000,B=0.221063,A=1.000000)" _color) :!class /Script/Engine.MaterialInstanceDynamic)
          (Rendering|Material|SetScalarParameterValue _dm_wall "Emissive" (Math|Float|Lerp 0.1 0.25 _color) :!class /Script/Engine.MaterialInstanceDynamic))
        (:Finished
          (CallFunction|ResetHit))))))

(event Custom|ResetHit
  (bind _dm_wall (Variables|Default|GetDM_Wall))
  (Utilities|FlowControl|DoOnce false) ; enters at Reset
)

(event EventBeginPlay
  (bind _plane (Variables|Default|GetPlane))
  (Utilities|FlowControl|Delay 0.3)
  (bind _returnvalue (Actor|GetActorOfClass "/Game/01_Character/Blueprints/BP_FirstPersonGameMode.BP_FirstPersonGameMode_C"))
  (Variables|Default|SetGameMode _returnvalue)
  (bind _returnvalue_2 (Actor|GetActorOfClass "/Game/01_Character/Blueprints/00_Character/BP_Character_P1.BP_Character_P1_C"))
  (Variables|Default|SetP1 _returnvalue_2)
  (Variables|Default|SetP1Bool true)
  (bind _returnvalue_3 (Actor|GetActorOfClass "/Game/01_Character/Blueprints/00_Character/BP_Character_P2.BP_Character_P2_C"))
  (Variables|Default|SetP2 _returnvalue_3)
  (Variables|Default|SetP2Bool true)
  (bind _returnvalue_4 (Rendering|Material|CreateDynamicMaterialInstance _plane 0 (Rendering|Material|GetMaterial _plane 0) "None" :!class /Script/Engine.PrimitiveComponent))
  (bind _output_get (Variables|Default|SetDM_Wall _returnvalue_4))
  (Rendering|Material|SetMaterial (Variables|Default|GetPlane) 0 _output_get))

(fn ConstructionScript)