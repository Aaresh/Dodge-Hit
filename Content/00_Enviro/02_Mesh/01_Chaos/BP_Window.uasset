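; Breakable Chaos window that shatters when a disc or explosion actor overlaps its sphere trigger.
; On a hit it enables physics on the geometry collection, spawns a master field at its location and disables collision.
; After a delay it destroys the original window component.
; ResetWindow re-enables collision and adds a new, non-simulating geometry collection as the active window, though the delayed destroy still targets the original.
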(event OnComponentBeginOverlap(Sphere)
  (params (OverlappedComponent :type Primitive%20Component%20Object%20Reference) (OtherActor :type Actor%20Object%20Reference) (OtherComp :type Primitive%20Component%20Object%20Reference) (OtherBodyIndex :type Integer) (bFromSweep :type Boolean) (SweepResult :type Hit%20Result%20Structure%20%28by%20ref%29))
  (bind _returnvalue (Utilities|GetClass OtherActor))
  (if (Math|Boolean|ORBoolean (== _returnvalue "/Game/01_Character/Blueprints/00_Character/BP_DiscManager.BP_DiscManager_C") (== _returnvalue "/Game/01_Character/Blueprints/00_Character/BP_DiscP1.BP_DiscP1_C") (== _returnvalue "/Game/01_Character/Blueprints/00_Character/BP_DiscP2.BP_DiscP2_C") (== "/Game/01_Character/Blueprints/BP_Explosion.BP_Explosion_C" _returnvalue) (== _returnvalue "/Game/01_Character/Blueprints/BP_Explosion_FromP1.BP_Explosion_FromP1_C") (== _returnvalue "/Game/01_Character/Blueprints/BP_Explosion_FromP2.BP_Explosion_FromP2_C"))
    (Physics|SetSimulatePhysics (Variables|Default|GetWINDOW) true)
    (Game|SpawnActorfromClass "/Engine/EditorResources/FieldNodes/FS_MasterField.FS_MasterField_C" (Math|Conversions|ToTransform(Vector) (Transformation|GetActorLocation)) "Undefined" "MultiplyWithRoot" 0 0)
    (Collision|SetCollisionEnabled (Variables|Default|GetCOLISION) "NoCollision")
    (Utilities|FlowControl|Delay 2.5)
    (Components|DestroyComponent (Variables|Default|GetGC_Chaos_Window_02))))

(event Custom|ResetWindow
  (Collision|SetCollisionEnabled (Variables|Default|GetCOLISION) "QueryAndProbe")
  (bind _returnvalue (AddComponent|AddGeometryCollectionComponent false))
  (bind _output_get (Variables|Default|SetWINDOW _returnvalue))
  (Physics|SetSimulatePhysics _output_get false))

(event EventBeginPlay
  (Variables|Default|SetWINDOW (Variables|Default|GetGC_Chaos_Window_02))
  (Physics|SetSimulatePhysics (Variables|Default|GetWINDOW) false))

(fn ConstructionScript)