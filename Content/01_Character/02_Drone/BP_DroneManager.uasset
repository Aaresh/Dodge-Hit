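; Sandbox drone actor with a hittable target plane that awards a point and respawns after a short delay.
; A looping timer turns the drone mesh in yaw to face player one, whose location is cached each Tick from the sandbox game mode.
; A hit plays the Appear timeline on the plane's dynamic material, then disables collision until respawn reverses it.
; A Respawn flag stops the reversed timeline's Finished from retriggering the cycle.
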(event OnComponentHit(Plane)
  (params (HitComponent :type Primitive%20Component%20Object%20Reference) (OtherActor :type Actor%20Object%20Reference) (OtherComp :type Primitive%20Component%20Object%20Reference) (NormalImpulse :type Vector :default "0, 0, 0") (Hit :type Hit%20Result%20Structure%20%28by%20ref%29))
  (Default|AddPoint (Variables|Default|GetGamemodeSandBox))
  (Variables|Default|SetRespawn%20? false)
  (bind _newtrack_0 (Timeline|Appear PlayFromStart)
    (:Update
      (Rendering|Material|SetScalarParameterValue (Variables|Default|GetDM_Target) "Visual" _newtrack_0 :!class /Script/Engine.MaterialInstanceDynamic))
    (:Finished
      (if (not (Variables|Default|GetRespawn%20?))
        (Collision|SetCollisionEnabled (Variables|Default|GetPlane) "NoCollision")
        (Utilities|FlowControl|Delay 3.0)
        (Variables|Default|SetRespawn%20? true)
        (CallFunction|Respawn)))))

(event Custom|Respawn
  (Collision|SetCollisionEnabled (Variables|Default|GetPlane) "QueryAndPhysics")
  (bind _newtrack_0 (Timeline|Appear ReverseFromEnd)
    (:Update
      (Rendering|Material|SetScalarParameterValue (Variables|Default|GetDM_Target) "Visual" _newtrack_0 :!class /Script/Engine.MaterialInstanceDynamic))
    (:Finished
      (if (not (Variables|Default|GetRespawn%20?))
        (Collision|SetCollisionEnabled (Variables|Default|GetPlane) "NoCollision")
        (Utilities|FlowControl|Delay 3.0)
        (Variables|Default|SetRespawn%20? true)
        (CallFunction|Respawn)))))

(event Custom|Rotation
  (bind _p1location (Variables|Default|GetP1Location))
  (bind _sm_drone (Variables|Default|GetSM_Drone))
  (bind _returnvalue (Transformation|GetWorldLocation _sm_drone))
  (bind _returnvalue_2 (Math|Rotator|FindLookatRotation _returnvalue _p1location))
  (bind (_roll _pitch _yaw) (Math|Rotator|BreakRotator _returnvalue_2))
  (Transformation|SetWorldRotation (Variables|Default|GetSM_Drone) (Math|Rotator|MakeRotator _roll 0.0 (- _yaw 9e+01)) false false))

(event EventBeginPlay
  (bind _plane (Variables|Default|GetPlane))
  (bind _returnvalue (Rendering|Material|CreateDynamicMaterialInstance _plane 0 (Rendering|Material|GetMaterial _plane 0) "None" :!class /Script/Engine.PrimitiveComponent))
  (Variables|Default|SetDM_Target _returnvalue)
  (bind _outactors (Actor|GetAllActorsOfClass "/Game/01_Character/Blueprints/BP_SandBoxGameMode.BP_SandBoxGameMode_C"))
  (Variables|Default|SetGamemodeSandBox (Utilities|Array|Get(acopy) _outactors))
  (Utilities|Time|SetTimerbyEvent (delegate Custom|Rotation) 0.01 true)
  (Variables|Default|SetP1 (Variables|/Game/01_Character/Blueprints/BP_SandBoxGameMode.BP_SandBoxGameMode_C|GetP1 (Variables|Default|GetGamemodeSandBox))))

(event EventTick
  (params (DeltaSeconds :type Float%20%28single-precision%29))
  (Variables|Default|SetP1Location (.location (Transformation|GetActorTransform (Variables|/Game/01_Character/Blueprints/BP_SandBoxGameMode.BP_SandBoxGameMode_C|GetP1 (Variables|Default|GetGamemodeSandBox))))))

(fn ConstructionScript)