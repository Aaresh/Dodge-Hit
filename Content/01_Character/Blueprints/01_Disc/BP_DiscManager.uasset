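; Thrown disc logic for a two-player game, resolving catches, player hits and surface impacts for BP_DiscP1 and BP_DiscP2.
; PlayerHit overlaps compare disc class and touched player: own disc re-enables that player's shot, opponent's disc reports a hit to the game mode, both destroying it.
; Concrete destroys the disc, Plastic adds Niagara effects and counts bounces without an active limit.
; Other blocking hits use a duplicate outcome check, wired only for surface misses.
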(event OnComponentBeginOverlap(PlayerHit)
  (params (OverlappedComponent :type Primitive%20Component%20Object%20Reference) (OtherActor :type Actor%20Object%20Reference) (OtherComp :type Primitive%20Component%20Object%20Reference) (OtherBodyIndex :type Integer) (bFromSweep :type Boolean) (SweepResult :type Hit%20Result%20Structure%20%28by%20ref%29))
  (bind _game_mode (Variables|Default|GetGame%20Mode))
  (Development|PrintString (Utilities|GetDisplayName OtherActor))
  (|Check_Outcome_2 (Utilities|GetClass self) OtherActor
    (:Catch%20P1
      (Development|PrintString "C1" true true "(R=1.000000,G=0.026842,B=0.000000,A=1.000000)")
      (Variables|/Game/01_Character/Blueprints/00_Character/BP_CharacterP1.BP_CharacterP1_C|SetIs_ShotValid (Variables|Default|GetP1) true))
    (:Mort%20P2
      (Development|PrintString "M2" true true "(R=1.000000,G=0.108599,B=0.000000,A=1.000000)")
      (Default|Player2Hit _game_mode))
    (:Mort%20P1
      (Development|PrintString "M1" true true "(R=1.000000,G=0.204350,B=0.000000,A=1.000000)")
      (Default|Player1Hit _game_mode))
    (:Catch%20P2
      (Development|PrintString "C2" true true "(R=1.000000,G=0.125463,B=0.000000,A=1.000000)")
      (Variables|/Game/01_Character/Blueprints/00_Character/BP_CharacterP2.BP_CharacterP2_C|SetIs_ShotValid (Variables|Default|GetP2) true)))
  (CallFunction|DestroyDisc))

(event Custom|DestroyDisc
  ;[0.15 0.15 0.15 0.5] destroy actor
  (Actor|DestroyActor)
  (Utilities|FlowControl|DoOnce false :!label _label
    (:Completed
      (AddComponent|AddNiagaraComponent false)
      (Utilities|FlowControl|Delay 0.2)
      (goto _label Reset))))

(event EventBeginPlay
  (bind _returnvalue (Actor|GetActorOfClass "/Game/01_Character/Blueprints/BP_FirstPersonGameMode.BP_FirstPersonGameMode_C"))
  (Variables|Default|SetGame%20Mode _returnvalue)
  (bind _returnvalue_2 (Actor|GetActorOfClass "/Game/01_Character/Blueprints/00_Character/BP_CharacterP1.BP_CharacterP1_C"))
  (Variables|Default|SetP1 _returnvalue_2)
  (bind _returnvalue_3 (Actor|GetActorOfClass "/Game/01_Character/Blueprints/00_Character/BP_CharacterP2.BP_CharacterP2_C"))
  (Variables|Default|SetP2 _returnvalue_3))

(event Collision|EventHit
  (params (MyComp :type Primitive%20Component%20Object%20Reference) (Other :type Actor%20Object%20Reference) (OtherComp :type Primitive%20Component%20Object%20Reference) (bSelfMoved :type Boolean) (HitLocation :type Vector :default "0, 0, 0") (HitNormal :type Vector :default "0, 0, 0") (NormalImpulse :type Vector :default "0, 0, 0") (Hit :type Hit%20Result%20Structure%20%28by%20ref%29))
  (if (Actor|ActorHasTag Other "Concrete")
    (CallFunction|DestroyDisc)
    (elif (Actor|ActorHasTag Other "Plastic")
      (AddComponent|AddNiagaraComponent false)
      (bind _result (Math|Integer|IncrementInt (Variables|Default|GetBounceNB))
        (:%20%20
          (Variables|Default|SetBounceNB _result)))
      (else
        (|Check_Outcome MyComp Other
          (:Touche%20surface
            (Development|PrintString "ca touche rien" true true "(R=0.000000,G=0.000000,B=0.000000,A=1.000000)")
            ;[0.15 0.15 0.15 0.5] Bounce
            (Rendering|Debug|DrawDebugCapsule (Transformation|GetActorLocation) 5e+01 5e+01 "0, 0, 0" "(R=1.000000,G=0.038864,B=0.000000,A=1.000000)" 1e+01 3.0)
            (CallFunction|DestroyDisc)))))))

(fn ConstructionScript)