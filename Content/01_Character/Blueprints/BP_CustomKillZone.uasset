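; Kill zone actor that reports when player 1 or player 2 enters its box to the first-person game mode.
; Shortly after BeginPlay it caches the game mode and both character actors.
; Box overlap calls the matching player-hit function, then a shared DoOnce triggers OutZoneDeath and resets after a delay.
; The death location comes from the empty component-hit event's output; other overlapping actors only print debug text.
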(event OnComponentBeginOverlap(Box)
  (params (OverlappedComponent :type Primitive%20Component%20Object%20Reference) (OtherActor :type Actor%20Object%20Reference) (OtherComp :type Primitive%20Component%20Object%20Reference) (OtherBodyIndex :type Integer) (bFromSweep :type Boolean) (SweepResult :type Hit%20Result%20Structure%20%28by%20ref%29))
  (bind _gamemode (Variables|Default|GetGameMode))
  (if (== OtherActor (Variables|Default|GetP1))
    (Default|Player1Hit _gamemode)
    (Utilities|FlowControl|DoOnce false :!label _label
      (:Completed
        (Default|OutZoneDeath (Variables|Default|GetGameMode) (.Location (Collision|BreakHitResult (stale OnComponentHit(Box) Hit))))
        (Utilities|FlowControl|Delay 2.0)
        (goto _label Reset)))
    (elif (== OtherActor (Variables|Default|GetP2))
      (Default|Player2Hit _gamemode)
      (goto _label)
      (else
        (Development|PrintString "Hello 44")))))

(event OnComponentHit(Box)
  (params (HitComponent :type Primitive%20Component%20Object%20Reference) (OtherActor :type Actor%20Object%20Reference) (OtherComp :type Primitive%20Component%20Object%20Reference) (NormalImpulse :type Vector :default "0, 0, 0") (Hit :type Hit%20Result%20Structure%20%28by%20ref%29)))

(event EventBeginPlay
  (Utilities|FlowControl|Delay 0.3)
  (bind _returnvalue (Actor|GetActorOfClass "/Game/01_Character/Blueprints/BP_FirstPersonGameMode.BP_FirstPersonGameMode_C"))
  (Variables|Default|SetGameMode _returnvalue)
  (bind _returnvalue_2 (Actor|GetActorOfClass "/Game/01_Character/Blueprints/00_Character/BP_Character_P1.BP_Character_P1_C"))
  (Variables|Default|SetP1 _returnvalue_2)
  (Variables|Default|SetP1Bool true)
  (bind _returnvalue_3 (Actor|GetActorOfClass "/Game/01_Character/Blueprints/00_Character/BP_Character_P2.BP_Character_P2_C"))
  (Variables|Default|SetP2 _returnvalue_3)
  (Variables|Default|SetP2Bool true))

(fn ConstructionScript)