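; Box trigger actor that destroys discs entering it and registers a hit on either player character that touches it.
; On begin overlap it checks the other actor's exact class: a BP_DiscManager is destroyed, then DiscDestroy_NS adds four Niagara components on it.
; For BP_CharacterP1 or P2, it clears FakeDisk on the game mode cached at BeginPlay and calls that player's hit function.
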(event OnComponentBeginOverlap(Box)
  (params (OverlappedComponent :type Primitive%20Component%20Object%20Reference) (OtherActor :type Actor%20Object%20Reference) (OtherComp :type Primitive%20Component%20Object%20Reference) (OtherBodyIndex :type Integer) (bFromSweep :type Boolean) (SweepResult :type Hit%20Result%20Structure%20%28by%20ref%29))
  (bind _returnvalue (Utilities|GetClass OtherActor))
  (bind _gamemode (Variables|Default|GetGameMode))
  (if (== _returnvalue "/Game/01_Character/Blueprints/00_Character/BP_DiscManager.BP_DiscManager_C")
    (Actor|DestroyActor OtherActor)
    (|DiscDestroy_NS OtherActor)
    (elif (== _returnvalue "/Game/01_Character/Blueprints/00_Character/BP_CharacterP1.BP_CharacterP1_C")
      (Variables|/Game/01_Character/Blueprints/BP_FirstPersonGameMode.BP_FirstPersonGameMode_C|SetFakeDisk _gamemode false)
      (Default|Player1Hit _gamemode)
      (elif (== _returnvalue "/Game/01_Character/Blueprints/00_Character/BP_CharacterP2.BP_CharacterP2_C")
        (Variables|/Game/01_Character/Blueprints/BP_FirstPersonGameMode.BP_FirstPersonGameMode_C|SetFakeDisk _gamemode false)
        (Default|Player2Hit _gamemode)))))

(event EventBeginPlay
  (bind _returnvalue (Actor|GetActorOfClass "/Game/01_Character/Blueprints/BP_FirstPersonGameMode.BP_FirstPersonGameMode_C"))
  (Variables|Default|SetGameMode _returnvalue))

(fn ConstructionScript)