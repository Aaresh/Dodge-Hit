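; BP_NotDestructibleFloor is a floor Blueprint whose events and construction script are all empty, so its graphs do nothing at runtime.
; Disconnected leftover logic describes a destructible floor: a timeline drives dissolve material parameters, disables collision, fires Niagara, hides the mesh, then calls Reparation after a delay.
; Other unwired chains lower the floor until Destruction, restore it raised above its start location, and jitter a cube's rotation.
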(event Custom|Destruction)

(event Custom|Degatdegat)

(event Custom|Reparation)

(event Custom|Moove)

(event EventBeginPlay)

(fn ConstructionScript)