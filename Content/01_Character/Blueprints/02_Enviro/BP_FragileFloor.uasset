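; BP_FragileFloor is a breakable floor that dissolves away when destroyed and can be restored by a repair event.
; BeginPlay creates a dynamic material, and both it and the damage event play the ActorHit sequence.
; Destruction swaps to that material, animates its dissolve on a Timeline, disables collision, fires Niagara through a DoOnce, then hides the mesh.
; Repair restores collision, visibility and material, and re-arms the DoOnce.
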(event Custom|Destruction
  (Rendering|Material|SetMaterial (Variables|Default|GetVisual_Animated) 0 (Variables|VFX|GetDM_Destruction))
  (Utilities|FlowControl|Sequence
    (:then_0
      (bind _timedissolution (Timeline|Timeline PlayFromStart)
        (:Update
          (Rendering|Material|SetScalarParameterValue (Variables|VFX|GetDM_Destruction) "TimeDissolution" _timedissolution :!class /Script/Engine.MaterialInstanceDynamic)
          (Collision|SetActorEnableCollision false)
          (Utilities|FlowControl|DoOnce false
            (:Completed
              (Components|Activation|Activate (Variables|Default|GetNS_FragileFloor) false))))
        (:Finished
          (Development|SetHiddeninGame (Variables|Default|GetVisual_Animated) true true)
          (Variables|Default|SetALIVE false))))
    (:then_1
      (Utilities|FlowControl|Delay 0.5))))

(event Custom|Degatdegat
  (Class|ActorSequenceComponent|PlaySequence (Variables|Default|GetActor_Hit)))

(event Custom|Reparation
  (if (not (Variables|Default|GetALIVE))
    (Utilities|FlowControl|Sequence
      (:then_0
        (Collision|SetActorEnableCollision true)
        (Development|SetHiddeninGame (Variables|Default|GetVisual_Animated) false true)
        (Variables|Default|SetALIVE true)
        (Rendering|Material|SetMaterial (Variables|Default|GetVisual_Animated) 0 "/Game/00_ValidatedEnviro/AssetPack/AssetPack_05/HexagonPlatform/Mi_Platform.Mi_Platform")
        (Rendering|Material|SetScalarParameterValue (Variables|VFX|GetDM_Destruction) "TimeDissolution" 0.0 :!class /Script/Engine.MaterialInstanceDynamic))
      (:then_1
        (Utilities|FlowControl|DoOnce false) ; enters at Reset
      ))))

(event EventBeginPlay
  (bind _ref_vfx (Variables|Default|GetRef_VFX))
  (Class|ActorSequenceComponent|PlaySequence (Variables|Default|GetActor_Hit))
  (bind _returnvalue (Rendering|Material|CreateDynamicMaterialInstance _ref_vfx 0 "/Game/00_ValidatedEnviro/AssetPack/AssetPack_05/HexagonPlatform/Mi_Platform.Mi_Platform" "None" :!class /Script/Engine.PrimitiveComponent))
  (Variables|VFX|SetDM_Destruction _returnvalue)
  (Variables|Default|SetMainMaterial (Rendering|Material|GetMaterial _ref_vfx 0)))

(fn ConstructionScript)