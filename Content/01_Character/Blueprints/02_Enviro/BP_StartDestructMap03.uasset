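; Environment actor that endlessly moves vertically between two Z limits, pausing at each end, with MinLocation serving as the upper limit despite its name.
; BeginPlay sets that limit from StartUp, which also forces a downward first move, then waits a short random delay before calling Restart.
; Restart alternates looping MooveUp and MooveDown timers that step the root with sweep.
; Timers are never cleared, so moving flags block the opposite direction and DoOnce gates schedule each delayed reversal.
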(event Custom|MooveUp
  (bind _defaultsceneroot (Variables|Default|GetDefaultSceneRoot))
  (bind _returnvalue (Transformation|GetWorldLocation _defaultsceneroot))
  (if (not (Variables|Default|GetIsMoovingDown))
    (if (>= (.Z (Math|Vector|BreakVector _returnvalue)) (Variables|Default|GetMinLocation))
      (Utilities|FlowControl|DoOnce false
        (:Completed
          (Utilities|FlowControl|Delay (Variables|Default|GetDealyBeforeRemove))
          (CallFunction|Restart)
          (Variables|Default|SetIsMoovingUp false)))
      (else
        (bind _output_get (Variables|Default|SetNewLocation (+ _returnvalue "0.000000,0.000000,1.000000")))
        (Transformation|SetWorldLocation (Variables|Default|GetDefaultSceneRoot) _output_get true false)
        (Variables|Default|SetIsMoovingUp true)))))

(event Custom|Restart
  (if (Variables|Default|GetUp&Down)
    (Utilities|Time|SetTimerbyFunctionName 0 "MooveUp" 0.01 true)
    (Variables|Default|SetUp&Down false)
    (Utilities|FlowControl|DoOnce false) ; enters at Reset
    (else
      (Utilities|Time|SetTimerbyFunctionName 0 "MooveDown" 0.01 true)
      (Variables|Default|SetUp&Down true)
      (Utilities|FlowControl|DoOnce false) ; enters at Reset
    )))

(event Custom|MooveDown
  (bind _defaultsceneroot (Variables|Default|GetDefaultSceneRoot))
  (bind _returnvalue (Transformation|GetWorldLocation _defaultsceneroot))
  (if (not (Variables|Default|GetIsMoovingUp))
    (if (<= (.Z (Math|Vector|BreakVector _returnvalue)) (Variables|Default|GetMaxLocation))
      (Utilities|FlowControl|DoOnce false
        (:Completed
          (Utilities|FlowControl|Delay (Variables|Default|GetDealyBeforeRemove))
          (CallFunction|Restart)
          (Variables|Default|SetIsMoovingDown false)))
      (else
        (bind _output_get (Variables|Default|SetNewLocation (- _returnvalue "0.000000,0.000000,1.000000")))
        (Transformation|SetWorldLocation (Variables|Default|GetDefaultSceneRoot) _output_get true false)
        (Variables|Default|SetIsMoovingDown true)))))

(event EventBeginPlay
  (if (Variables|Default|GetStartUp)
    (Variables|Default|SetUp&Down false)
    (Variables|Default|SetMinLocation -1335.0)
    (else
      (Variables|Default|SetMinLocation -1.58e+03)))
  (Variables|Default|SetStartLocation (Transformation|GetWorldLocation (Variables|Default|GetDefaultSceneRoot)))
  (Variables|Default|SetFirstMoove (Math|Random|RandomFloatinRange 0.0 2.0))
  (Utilities|FlowControl|Delay (Variables|Default|GetFirstMoove))
  (CallFunction|Restart))

(event EventTick
  (params (DeltaSeconds :type Float%20%28single-precision%29)))

(fn ConstructionScript)