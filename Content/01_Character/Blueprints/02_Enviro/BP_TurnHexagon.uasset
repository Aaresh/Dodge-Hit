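; BP_TurnHexagon is an environment Blueprint that continuously spins its TurnPropler component in world space once StartTurn is called.
; StartTurn caches the component's world rotation and starts a looping timer on the Turn function at the RotationRate interval, avoiding Tick.
; Each Turn call combines a small fixed yaw step into the stored rotation and applies it, so RotationRate sets the spin speed.
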(event Custom|Turn
  (if true
    (bind _output_get (Variables|Default|SetCurrentRotation (Math|Rotator|CombineRotators (Variables|Default|GetCurrentRotation) (Math|Rotator|MakeRotator 0.0 0.0 0.05))))
    (Transformation|SetWorldRotation (Variables|Default|GetTurnPropler) _output_get false false)))

(event Custom|StartTurn
  (bind _output_get (Variables|Default|SetStartWorldRotation (Transformation|GetWorldRotation (Variables|Default|GetTurnPropler))))
  (Variables|Default|SetCurrentRotation _output_get)
  (Utilities|Time|SetTimerbyFunctionName 0 "Turn" (Variables|Default|GetRotationRate) true))

(fn ConstructionScript)