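; Space station actor that gives two player characters custom gravity, cached at BeginPlay after a delay.
; Each tick it turns P1's root along the look-at from a Start point, with a 90-degree offset.
; ArrowP1 follows that look-at with pitch flattened, so its forward vector pulls P1 radially outward as gravity.
; P2's gravity follows ArrowP2's forward vector, but only ArrowP1 and P1 are rotated here.
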(event EventTick
  (params (DeltaSeconds :type Float%20%28single-precision%29))
  (bind _characterp1 (Variables|Default|GetCharacterP1))
  (bind _start (Variables|Default|GetStart))
  (bind _characterp1_2 (Variables|Default|GetCharacterP1))
  (bind _start_2 (Variables|Default|GetStart))
  (bind _returnvalue (Transformation|GetActorLocation _characterp1))
  (bind _returnvalue_2 (Transformation|GetActorLocation _characterp1_2))
  (bind _returnvalue_3 (Math|Rotator|FindLookatRotation _start_2 _returnvalue))
  (bind _returnvalue_4 (Math|Rotator|FindLookatRotation _start _returnvalue_2))
  (bind (_roll _pitch _yaw) (Math|Rotator|BreakRotator _returnvalue_3))
  (bind (_roll_2 _pitch_2 _yaw_2) (Math|Rotator|BreakRotator _returnvalue_4))
  (Transformation|SetRelativeRotation (Variables|/Script/Engine.Actor|GetRootComponent (Variables|Default|GetCharacterP1)) (Math|Rotator|CombineRotators _returnvalue_4 "-90.000000,0.000000,90.000000") false false)
  (Transformation|SetWorldRotation (Variables|Default|GetArrow_P1) (Math|Rotator|MakeRotator _roll_2 0.0 _yaw_2) false false)
  (Transformation|SetWorldRotation (Variables|Default|GetArrow_P1) (Math|Rotator|MakeRotator _roll 0.0 _yaw) false false)
  (Class|CharacterMovementComponent|SetGravityDirection (Variables|/Script/Engine.Character|GetCharacterMovement (Variables|Default|GetCharacterP1)) (Math|Vector|GetForwardVector (Variables|Default|GetArrow_P1)))
  (Class|CharacterMovementComponent|SetGravityDirection (Variables|/Script/Engine.Character|GetCharacterMovement (Variables|Default|GetCharacterP2)) (Math|Vector|GetForwardVector (Variables|Default|GetArrow_P2))))

(event EventBeginPlay
  (Utilities|FlowControl|Delay (stale EventTick DeltaSeconds))
  (bind _returnvalue (Actor|GetActorOfClass "/Game/01_Character/Blueprints/00_Character/BP_Character_P1.BP_Character_P1_C"))
  (Variables|Default|SetCharacterP1 _returnvalue)
  (bind _returnvalue_2 (Actor|GetActorOfClass "/Game/01_Character/Blueprints/00_Character/BP_Character_Manager.BP_Character_Manager_C"))
  (Variables|Default|SetCharacterP2 _returnvalue_2))

(fn ConstructionScript)