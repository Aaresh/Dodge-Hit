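; Cosmetic robot explosion actor that leaves a randomly sized scorch decal at its location and flashes a point light.
; On BeginPlay, one timeline dims the light before destroying it, while a second animates the decal's alpha and then starts a delayed fade-out.
; Two layered 2D explosion sounds play once on the light timeline's first update, only when FromReplayDisc is set.
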(event EventBeginPlay
  (bind _returnvalue (Rendering|Decal|SpawnDecalatLocation "/Game/03_VFX/02_Material/DiskExplode/Mi_DiskExplosionDecal_P2.Mi_DiskExplosionDecal_P2" (* (Math|Vector|MakeVector (Math|Random|RandomFloatinRange 0.8 1.2) (Math|Random|RandomFloatinRange 0.8 1.2) 1.0) (Math|Random|RandomFloatinRange 2e+02 3e+02)) (Transformation|GetActorLocation) "-90.000000,0.000000,0.000000" 0.0))
  (Variables|Default|SetDecalComponent _returnvalue)
  (Utilities|FlowControl|Sequence
    (:then_0
      (bind _intensity (Timeline|Timeline PlayFromStart)
        (:Update
          (Rendering|Components|Light|SetIntensity (Variables|Default|GetPointLight) (Math|Float|Lerp 1e+01 0.0 _intensity))
          (Utilities|FlowControl|DoOnce false
            (:Completed
              ;[1 0 0.6076 0.5 75] SONS
              (if (Variables|Default|GetFromReplayDisc)
                (Audio|SpawnSound2D "/Game/05_SONS/Disque/OLD/Explosion_Basse.Explosion_Basse" 0.5 1.0 0.0 0)
                (Audio|SpawnSound2D "/Game/05_SONS/Disque/OLD/Explosion_Texture.Explosion_Texture" 0.3 1.0 0.0 0)))))
        (:Finished
          (Components|DestroyComponent (Variables|Default|GetPointLight)))))
    (:then_1
      (bind _intensity_2 (Timeline|Timeline_0 PlayFromStart)
        (:Update
          (Rendering|Components|Decal|SetDecalColor (Variables|Default|GetDecalComponent) (Utilities|Struct|MakeLinearColor 0.0 0.0 0.0 _intensity_2)))
        (:Finished
          (Rendering|Components|Decal|SetFadeOut (Variables|Default|GetDecalComponent) 2.0 4.0 true))))))

(fn ConstructionScript)