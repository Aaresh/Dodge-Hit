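; Main menu game mode that creates a local player for each PlayerStart in the level.
; On BeginPlay it loops over the PlayerStart actors, passing each array index to CreatePlayer.
; Disconnected leftover graphs would play the Cinematic_WakeUp sequence with both player controllers viewing the CAM1 camera, or repeatedly show a timed media player widget, but neither runs.
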(event EventBeginPlay
  (bind _outactors (Actor|GetAllActorsOfClass "/Script/Engine.PlayerStart"))
  (for (_ _array_index) _outactors
    (bind _output_get (Variables|Default|SetArray%20Index _array_index))
    (Class|GameplayStatics|CreatePlayer _output_get)))

(fn ConstructionScript)