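; Game mode for a sandbox level that spawns and possesses the player 1 character at a player start, sets its input mapping, then disables its input.
; Helper functions reset rounds, toggle look and move input for two controllers, store death and shot positions, and take dead players offline with a fade and follow-camera timer.
; Kill-cam functions point both views at a tagged camera near the dead player, falling back to a main kill camera.
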(event EventBeginPlay
  (bind _returnvalue (Game|GetPlayerController 0))
  (bind _returnvalue_2 (Game|GetPlayerController 0))
  (bind _returnvalue_3 (PlayerController|LocalPlayerSubsystems|GetEnhancedInputLocalPlayerSubsystem _returnvalue))
  ;[1 0.05729 0.05729 0.5 50] BeginPlay
  (|PostProcessVariable_2)
  (Variables|RoundSystem|SetRoundSet false)
  (bind _outactors (Actor|GetAllActorsOfClass "/Script/Engine.PlayerStart"))
  ;;[0.15 0.15 0.15 0.5] Are P2
  (Input|AddMappingContext _returnvalue_3 "/Game/01_Character/Input/IMC_GamePadP2.IMC_GamePadP2" 0 "(bIgnoreAllPressedKeysUntilRelease=True,bForceImmediately=False,bNotifyUserSettings=False)")
  (Input|RemoveMappingContext _returnvalue_3 "/Game/01_Character/Input/IMC_MenuInput.IMC_MenuInput" "(bIgnoreAllPressedKeysUntilRelease=True,bForceImmediately=False,bNotifyUserSettings=False)")
  (bind _returnvalue_4 (Game|SpawnActorfromClass "/Game/01_Character/Blueprints/00_Character/BP_Character_P1.BP_Character_P1_C" (Transformation|GetActorTransform (Utilities|Array|Get(acopy) _outactors)) "Undefined" "MultiplyWithRoot" 0 2.0 2.0 0))
  (Pawn|Possess (Game|GetPlayerController 0) _returnvalue_4)
  (Variables|Player|SetPlayer2_ID 0)
  (Utilities|FlowControl|Delay 0.1)
  (bind _returnvalue_5 (Actor|GetActorOfClass "/Game/01_Character/Blueprints/00_Character/BP_Character_P1.BP_Character_P1_C"))
  (bind _output_get (Variables|Player|SetP1 _returnvalue_5))
  (Variables|Player|SetWStartLocation%20P1 (Transformation|GetActorLocation _output_get))
  (Variables|Player|SetStartRotationRotationPlayer1 (Pawn|GetControlRotation (Game|Player|GetPlayerPawn 0) :!class /Script/Engine.Pawn))
  (Input|DisableInput (Variables|Player|GetP1) _returnvalue_2)
  (AI|Navigation|StopMovement _returnvalue_2)
  (Class|EnhancedInputLibrary|FlushPlayerInput _returnvalue_2)
  (Class|EnhancedInputSubsystemInterface|ClearAllMappings(Message) _returnvalue_2)
  (Variables|DeathCam|SetP1_ReplayCamera (Variables|/Game/01_Character/Blueprints/00_Character/BP_Character_Manager.BP_Character_Manager_C|GetReplayCamera (Variables|Player|GetP1))))

(fn ConstructionScript)

(fn ResetRound
  ;[0.15 0.15 0.15 0.5] RESET PLAYER VIEW
  (Utilities|Time|ClearandInvalidateTimerbyHandle (Variables|DeathCam|GetTimerDeathCam))
  (Game|Player|SetViewTargetwithBlend (Game|GetPlayerController 0) (Game|Player|GetPlayerPawn 0) 0.0 "VTBlend_Linear" 0.0 false)
  (Game|Player|SetViewTargetwithBlend (Game|GetPlayerController 1) (Game|Player|GetPlayerPawn 1) 0.0 "VTBlend_Linear" 0.0 false)
  (Variables|RoundSystem|SetRoundEnded false)
  (Utilities|Map|Clear (Variables|Player|GetCharacter%20and%20Pos))
  (Utilities|Map|Clear (Variables|Player|GetDisc%20and%20Pos))
  (Class|EnhancedInputLibrary|FlushPlayerInput (Game|GetPlayerController 0))
  (Class|EnhancedInputLibrary|FlushPlayerInput (Game|GetPlayerController 1))
  (if (Variables|RoundSystem|GetGameEnded)
    _))

(fn DisableMvnt/TPtoDeath
  (bind _p1 (Variables|Player|GetP1))
  (bind _charactermovement (Variables|/Script/Engine.Character|GetCharacterMovement _p1))
  (Variables|/Script/Engine.CharacterMovementComponent|SetGravityScale _charactermovement 0.0)
  (Pawn|Components|CharacterMovement|DisableMovement _charactermovement)
  (Class|EnhancedInputLibrary|FlushPlayerInput (Game|GetPlayerController 0))
  (Transformation|SetActorLocation _p1 (.Value (Utilities|Map|Find (Variables|Default|GetCharacter%20And%20Pos) "/Game/01_Character/Blueprints/00_Character/BP_Character_P1.BP_Character_P1_C")) false true)
  (return))

(fn ResearchClosestCameraReplay
  (bind _returnvalue (Game|GetPlayerController 0))
  (bind _outactors (Actor|GetAllActorswithTag "KillCam"))
  (bind _array_element (Utilities|Array|ForEachLoopwithBreak _outactors :!label _label)
    (:LoopBody
      (if (< (Math|Vector|Distance(Vector) (Transformation|GetActorLocation _array_element) (Transformation|GetActorLocation (Variables|DeathCam|GetPlayerDied))) 1.4e+03)
        (Utilities|FlowControl|Sequence
          (:then_0
            (bind _output_get (Variables|DeathCam|SetReplayCamera _array_element))
            (Game|Player|SetViewTargetwithBlend _returnvalue _output_get 0.0 "VTBlend_Linear" 0.0 false)
            (Transformation|SetActorRotation (Variables|DeathCam|GetReplayCamera) (Math|Rotator|FindLookatRotation (Transformation|GetActorLocation (Variables|DeathCam|GetReplayCamera)) (Transformation|GetActorLocation (Variables|DeathCam|GetPlayerDied)))))
          (:then_1
            (goto _label Break)))
        (else
          (bind _outactors_2 (Actor|GetAllActorswithTag "MainKillCam"))
          (bind _output_get_2 (Variables|DeathCam|SetReplayCamera (Utilities|Array|Get(acopy) _outactors_2)))
          (Game|Player|SetViewTargetwithBlend _returnvalue _output_get_2 0.0 "VTBlend_Linear" 0.0 false)
          (Transformation|SetActorRotation (Variables|DeathCam|GetReplayCamera) (Math|Rotator|FindLookatRotation (Transformation|GetActorLocation (Variables|DeathCam|GetReplayCamera)) (Transformation|GetActorLocation (Variables|DeathCam|GetPlayerDied)))))))))

(fn ResearchCameraReplayDirectHit
  (bind _returnvalue (Game|GetPlayerController 0))
  (bind _outactors (Actor|GetAllActorswithTag "KillCam"))
  (bind _array_element (Utilities|Array|ForEachLoopwithBreak _outactors :!label _label)
    (:LoopBody
      (if (< (Math|Vector|Distance(Vector) (Transformation|GetActorLocation _array_element) (Transformation|GetActorLocation (Variables|DeathCam|GetPlayerDied))) 1.4e+03)
        (Utilities|FlowControl|Sequence
          (:then_0
            (Variables|DeathCam|SetReplayCamera _array_element)
            (Game|Player|SetViewTargetwithBlend _returnvalue _array_element 0.0 "VTBlend_Linear" 0.0 false))
          (:then_1
            (goto _label Break)))
        (else
          (bind _outactors_2 (Actor|GetAllActorswithTag "MainKillCam"))
          (Variables|DeathCam|SetReplayCamera (Utilities|Array|Get(acopy) _outactors_2))
          (Game|Player|SetViewTargetwithBlend _returnvalue (Utilities|Array|Get(acopy) _outactors_2) 0.0 "VTBlend_Linear" 0.0 false))))))

(fn SetDeathPlayerandOppositePostion
  (params (PlayerDied :type Actor%20Object%20Reference) (P1PositionAtDeath :type Vector) (P2PositionAtDeath :type Vector) (P1RotationAtDeath :type Rotator) (P2RotationAtDeath :type Rotator))
  (Variables|DeathCam|SetPlayerDied PlayerDied)
  (Variables|DeathCam|SetP1PositionAtDeath P1PositionAtDeath))

(fn SaveLocationwhenShoot
  (Variables|DeathCam|SetP1_ShootPosition (.Value (Utilities|Map|Find (Variables|Player|GetCharacter%20and%20Pos) "/Game/01_Character/Blueprints/00_Character/BP_Character_P1.BP_Character_P1_C"))))

(fn SetPlayerOffline
  (params (Player%20Dead :type BP%20Character%20Manager%20Object%20Reference) (Replay%20Camera :type Actor%20Component%20Object%20Reference) (FunctionName :type String))
  (bind _returnvalue (UserInterface|CreateWidget "/Game/03_VFX/04_PlayerUI/WBP_BlackFade.WBP_BlackFade_C"))
  (UserInterface|Viewport|AddtoViewport _returnvalue 0)
  (Components|Activation|Deactivate (Variables|/Game/01_Character/Blueprints/00_Character/BP_Character_Manager.BP_Character_Manager_C|GetFirstPersonCamera Player%20Dead))
  (Input|DisableInput Player%20Dead (Game|GetPlayerController (select (== Player%20Dead "/Game/01_Character/Blueprints/00_Character/BP_Character_P1.BP_Character_P1") 0 1)))
  (Components|Activation|SetActive Replay%20Camera true false)
  (Default|Offline Player%20Dead)
  (bind _returnvalue_2 (Utilities|Time|SetTimerbyFunctionName 0 FunctionName 0.001 true))
  (Variables|DeathCam|SetTimerFollowCamera _returnvalue_2))

(fn ResetInput
  (Input|SetIgnoreLookInput (Game|GetPlayerController 0) true)
  (Input|SetIgnoreLookInput (Game|GetPlayerController 1) true)
  (Input|SetIgnoreMoveInput (Game|GetPlayerController 0) true)
  (Input|SetIgnoreMoveInput (Game|GetPlayerController 1) true))

(fn EnableInputReset
  (Input|SetIgnoreLookInput (Game|GetPlayerController 0) false)
  (Input|SetIgnoreLookInput (Game|GetPlayerController 1) false)
  (Input|SetIgnoreMoveInput (Game|GetPlayerController 0) false)
  (Input|SetIgnoreMoveInput (Game|GetPlayerController 1) false))