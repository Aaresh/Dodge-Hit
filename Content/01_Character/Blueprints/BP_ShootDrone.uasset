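; Drone that circles a looping spline and fires robot discs at one of the two players.
; Tick moves it along the spline while turning drone and arrow toward a snapshot of a randomly picked P1 or P2 homing actor location.
; Each shot plays an effect, then spawns BP_DiscRobot from the arrow.
; A looping timer polls until no disc remains, then schedules the next shot after a random delay.
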(event Custom|CheckForDisc
  (bind _returnvalue (Actor|GetActorOfClass "/Game/01_Character/Blueprints/00_Character/BP_DiscRobot.BP_DiscRobot_C"))
  (Utilities|IsValid _returnvalue
    (:Is%20Not%20Valid
      (Utilities|Time|ClearandInvalidateTimerbyHandle (stale Custom|ShootDisc _returnvalue))
      (Utilities|FlowControl|RetriggerableDelay (Math|Random|RandomFloatinRange 2.0 3.0))
      (CallFunction|ShootDisc))))

(event Custom|ShootDisc
  (Variables|Default|SetTargetLocation (Utilities|Select :Index (Math|Random|RandomIntegerinRange 0 1) :Option%200 (Variables|Default|GetP1Location) :Option%201 (Variables|Default|GetP2Location)))
  (Components|Activation|Activate (Variables|Default|GetNS_ShootDiscDrone) false)
  (Utilities|FlowControl|Delay 0.5)
  (Game|SpawnActorfromClass "/Game/01_Character/Blueprints/00_Character/BP_DiscRobot.BP_DiscRobot_C" (Transformation|GetWorldTransform (Variables|Default|GetArrow)) "AlwaysSpawn" "MultiplyWithRoot" self false "2250.000000,0.000000,0.000000" 1.25e+05 0)
  (bind _returnvalue (Utilities|Time|SetTimerbyEvent (delegate Custom|CheckForDisc) 0.01 true))
  (Utilities|FlowControl|Delay (Math|Random|RandomFloatinRange 4.0 5.0)))

(event EventBeginPlay
  (Utilities|FlowControl|Sequence
    (:then_0
      ;[0.15 0.15 0.15 0.5] GetValuePlayer
      (Utilities|FlowControl|Delay 1.0)
      (Variables|Default|SetStartMoove? true)
      (bind _returnvalue (Actor|GetActorOfClass "/Game/01_Character/Blueprints/00_Character/BP_HommingActorP1.BP_HommingActorP1_C"))
      (Variables|Default|SetP1 _returnvalue)
      (bind _returnvalue_2 (Actor|GetActorOfClass "/Game/01_Character/Blueprints/00_Character/BP_HommingActorP2.BP_HommingActorP2_C"))
      (Variables|Default|SetP2 _returnvalue_2))
    (:then_1
      (Utilities|FlowControl|Delay 7.5)
      (Variables|Default|SetTargetLocation (Utilities|Select :Index (Math|Random|RandomIntegerinRange 0 1) :Option%200 (Variables|Default|GetP1Location) :Option%201 (Variables|Default|GetP2Location)))
      (Components|Activation|Activate (Variables|Default|GetNS_ShootDiscDrone) false)
      (Utilities|FlowControl|Delay 0.5)
      (Game|SpawnActorfromClass "/Game/01_Character/Blueprints/00_Character/BP_DiscRobot.BP_DiscRobot_C" (Transformation|GetWorldTransform (Variables|Default|GetArrow)) "AlwaysSpawn" "MultiplyWithRoot" self false "2250.000000,0.000000,0.000000" 1.25e+05 0)
      (bind _returnvalue_3 (Utilities|Time|SetTimerbyEvent (delegate Custom|CheckForDisc) 0.01 true))
      (Utilities|FlowControl|Delay (Math|Random|RandomFloatinRange 4.0 5.0)))))

(event EventTick
  (params (DeltaSeconds :type Float%20%28single-precision%29))
  (bind _drone (Variables|Default|GetDrone))
  (bind _p1 (Variables|Default|GetP1))
  (Utilities|IsValid _p1
    (:Is%20Valid
      (Variables|Default|SetP1Location (Transformation|GetActorLocation _p1))
      (Variables|Default|SetP2Location (Transformation|GetActorLocation (Variables|Default|GetP2)))
      (Transformation|SetWorldRotation (Variables|Default|GetArrow) (Math|Rotator|FindLookatRotation (Transformation|GetWorldLocation (Variables|Default|GetDrone)) (Variables|Default|GetTargetLocation)) false false)
      (if (Variables|Default|GetStartMoove?)
        (bind _output_get (Variables|Default|SetDistanceAlongSpline (+ (* (* DeltaSeconds (Variables|Default|GetSpeed)) (Variables|Default|GetSpeedAlongSpline)) (Variables|Default|GetDistanceAlongSpline))))
        (Transformation|SetRelativeTransform _drone (Math|Transform|MakeTransform (.location (Spline|GetTransformatDistanceAlongSpline (Variables|Default|GetSpline) _output_get "Local" false)) (Math|Rotator|FindLookatRotation (Transformation|GetWorldLocation (Variables|Default|GetDrone)) (Variables|Default|GetTargetLocation)) (Variables|/Script/Engine.SceneComponent|GetRelativeScale3D _drone)) false false)
        (if (>= (Variables|Default|GetDistanceAlongSpline) (Spline|GetSplineLength (Variables|Default|GetSpline)))
          (Variables|Default|SetDistanceAlongSpline 0.0))))))

(fn ConstructionScript)