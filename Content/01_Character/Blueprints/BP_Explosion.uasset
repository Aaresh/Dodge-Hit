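; Explosion actor that plays two layered sounds and affects both players and fragile floors through two overlap radii.
; The death radius reports player hits to BP_FirstPersonGameMode and calls Destruction on BP_FragileFloor.
; The push radius launches a player away from the center by PushForce, then removes itself.
; With Explode set, both radii are removed after a brief delay and the actor destroys itself later; otherwise a player hit destroys it.
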(event OnComponentBeginOverlap(Death_Radius)
  (params (OverlappedComponent :type Primitive%20Component%20Object%20Reference) (OtherActor :type Actor%20Object%20Reference) (OtherComp :type Primitive%20Component%20Object%20Reference) (OtherBodyIndex :type Integer) (bFromSweep :type Boolean) (SweepResult :type Hit%20Result%20Structure%20%28by%20ref%29))
  (bind _returnvalue (Game|GetGameMode))
  (bind _returnvalue_2 (Utilities|GetClass OtherActor))
  (bind _game_mode (Variables|Default|GetGame%20Mode))
  (bind _defaultsceneroot (Variables|Default|GetDefaultSceneRoot))
  (bind _returnvalue_3 (Transformation|GetWorldLocation _defaultsceneroot))
  (if (== _returnvalue_2 "/Game/01_Character/Blueprints/00_Character/BP_Character_P1.BP_Character_P1_C")
    (Utilities|FlowControl|DoOnce false
      (:Completed
        (Variables|/Game/01_Character/Blueprints/BP_FirstPersonGameMode.BP_FirstPersonGameMode_C|SetFakeDisk _game_mode false)
        (Class|BPIDodgeHit|PlayerExplosionHit(Message) _returnvalue _returnvalue_3)
        (Variables|/Game/01_Character/Blueprints/BP_FirstPersonGameMode.BP_FirstPersonGameMode_C|SetDeathGround _game_mode true)
        (Default|Player1Hit _game_mode)
        (if (not (Variables|Default|GetExplode)) :!label _label
          (Components|DestroyComponent (Variables|Default|GetDeath_Radius))
          (Actor|DestroyActor))))
    (elif (== _returnvalue_2 "/Game/01_Character/Blueprints/00_Character/BP_Character_P2.BP_Character_P2_C")
      (Utilities|FlowControl|DoOnce false
        (:Completed
          (Variables|/Game/01_Character/Blueprints/BP_FirstPersonGameMode.BP_FirstPersonGameMode_C|SetFakeDisk _game_mode false)
          (Class|BPIDodgeHit|PlayerExplosionHit(Message) _returnvalue _returnvalue_3)
          (Variables|/Game/01_Character/Blueprints/BP_FirstPersonGameMode.BP_FirstPersonGameMode_C|SetDeathGround _game_mode true)
          (Default|Player2Hit _game_mode)
          (goto _label)))
      (elif (== _returnvalue_2 "/Game/01_Character/Blueprints/02_Enviro/BP_FragileFloor.BP_FragileFloor_C")
        (Utilities|IsValid OtherActor
          (:Is%20Valid
            (bind _asbp_fragile_floor (Utilities|Casting|CastToBP_FragileFloor OtherActor))
            (Default|Destruction _asbp_fragile_floor)))))))

(event OnComponentBeginOverlap(Push_Radius)
  (params (OverlappedComponent :type Primitive%20Component%20Object%20Reference) (OtherActor :type Actor%20Object%20Reference) (OtherComp :type Primitive%20Component%20Object%20Reference) (OtherBodyIndex :type Integer) (bFromSweep :type Boolean) (SweepResult :type Hit%20Result%20Structure%20%28by%20ref%29))
  (bind _returnvalue (Utilities|GetClass OtherActor))
  (bind _returnvalue_2 (Transformation|GetActorLocation))
  (bind _returnvalue_3 (Transformation|GetActorLocation))
  (bind _p2 (Variables|Default|GetP2))
  (bind _p1 (Variables|Default|GetP1))
  (bind _push_force (Variables|Default|GetPush_Force))
  (bind _returnvalue_4 (Transformation|GetActorLocation _p1))
  (bind _returnvalue_5 (Transformation|GetActorLocation _p2))
  (bind _returnvalue_6 (Math|Vector|GetUnitDirection(Vector) _returnvalue_2 _returnvalue_4))
  (bind _returnvalue_7 (Math|Vector|GetUnitDirection(Vector) _returnvalue_3 _returnvalue_5))
  (bind _returnvalue_8 (* _returnvalue_7 _push_force))
  (bind _returnvalue_9 (* _returnvalue_6 _push_force))
  (if (== _returnvalue "/Game/01_Character/Blueprints/00_Character/BP_Character_P1.BP_Character_P1_C")
    (Utilities|FlowControl|Sequence
      (:then_0
        (Utilities|FlowControl|DoOnce false
          (:Completed
            (Development|PrintString (Utilities|String|ToString(Vector) _returnvalue_9) true false "(R=0.000000,G=0.821211,B=1.000000,A=1.000000)" 1e+01)
            (Default|PUSHED (Variables|Default|GetP1) _returnvalue_9)
            (Components|DestroyComponent (Variables|Default|GetPush_Radius) :!label _label))))
      (:then_1
        (if (== _returnvalue "/Game/01_Character/Blueprints/00_Character/BP_Character_P2.BP_Character_P2_C") :!label _label_2
          (Utilities|FlowControl|DoOnce false
            (:Completed
              (Development|PrintString (Utilities|String|ToString(Vector) _returnvalue_8) true false "(R=1.000000,G=0.167941,B=0.000000,A=1.000000)" 1e+01)
              (Default|PUSHED (Variables|Default|GetP2) _returnvalue_8)
              (goto _label))))))
    (else
      (goto _label_2))))

(event EventBeginPlay
  (bind _push_radius (Variables|Default|GetPush_Radius))
  (bind _death_radius (Variables|Default|GetDeath_Radius))
  (bind _returnvalue (Actor|GetActorOfClass "/Game/01_Character/Blueprints/00_Character/BP_Character_P1.BP_Character_P1_C"))
  (Variables|Default|SetP1 _returnvalue)
  (bind _returnvalue_2 (Actor|GetActorOfClass "/Game/01_Character/Blueprints/00_Character/BP_Character_P2.BP_Character_P2_C"))
  (Variables|Default|SetP2 _returnvalue_2)
  ;[1 0 0.6076 0.5 75] SONS
  (Audio|SpawnSound2D "/Game/05_SONS/Disque/Explosion_Basse.Explosion_Basse" 0.5 1.0 0.0 0)
  (Audio|SpawnSound2D "/Game/05_SONS/Disque/Explosion_Texture.Explosion_Texture" 0.3 1.0 0.0 0)
  (if (Variables|Default|GetExplode)
    (bind _returnvalue_3 (Actor|GetActorOfClass "/Game/01_Character/Blueprints/BP_FirstPersonGameMode.BP_FirstPersonGameMode_C"))
    (Variables|Default|SetGame%20Mode _returnvalue_3)
    (Utilities|FlowControl|Delay 0.1)
    (Utilities|IsValid _push_radius
      (:Is%20Valid
        (Components|DestroyComponent _push_radius))
      (:Is%20Not%20Valid
        _))
    (Utilities|IsValid _death_radius
      (:Is%20Valid
        (Components|DestroyComponent _death_radius))
      (:Is%20Not%20Valid
        _))
    (Utilities|FlowControl|Delay 5.0)
    (Actor|DestroyActor)))

(fn ConstructionScript)