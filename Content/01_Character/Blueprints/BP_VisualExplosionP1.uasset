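; Visual explosion actor (P1 variant) that produces a brief light flash with optional explosion audio.
; On BeginPlay, a timeline drives the PointLight intensity from its curve, then destroys the light component, not the actor, when finished.
; A DoOnce on the timeline update plays two layered 2D explosion sounds, bass and texture, only when FromReplayDisc is set.
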(event EventBeginPlay
  (bind _intensity (Timeline|SetIntensity PlayFromStart)
    (:Update
      (Rendering|Components|Light|SetIntensity (Variables|Default|GetPointLight) (Math|Float|Lerp 5.0 0.0 _intensity))
      (Utilities|FlowControl|DoOnce false
        (:Completed
          (if (Variables|Default|GetFromReplayDisc)
            ;[1 0 0.6076 0.5 75] SONS
            (Audio|SpawnSound2D "/Game/05_SONS/Disque/OLD/Explosion_Basse.Explosion_Basse" 0.5 1.0 0.0 0)
            (Audio|SpawnSound2D "/Game/05_SONS/Disque/OLD/Explosion_Texture.Explosion_Texture" 0.3 1.0 0.0 0)))))
    (:Finished
      (Components|DestroyComponent (Variables|Default|GetPointLight)))))

(fn ConstructionScript)