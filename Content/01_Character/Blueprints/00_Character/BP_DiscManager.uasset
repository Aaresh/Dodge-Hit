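; BP_DiscManager is the shared logic for thrown discs (P1, P2, robot) in a two-player dodging game.
; It homes on a target actor with timeline-driven acceleration, shows target widgets, and sets local velocity each tick, zeroed during P1's pause menu.
; Player overlaps report kills to the game mode by disc class.
; Surface tags pick a re-homing bounce (Plastic) or explosion, while replay discs take separate, mostly visual branches.
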(event OnComponentHit(Collider_Replay)
  (params (HitComponent :type Primitive%20Component%20Object%20Reference) (OtherActor :type Actor%20Object%20Reference) (OtherComp :type Primitive%20Component%20Object%20Reference) (NormalImpulse :type Vector :default "0, 0, 0") (Hit :type Hit%20Result%20Structure%20%28by%20ref%29))
  ;[0.1529 0.15 0.5029 0.502] First Collision
  (if (Variables|02_DiskProperties|GetReplayDisc)
    (if (not (== (Components|GetOwner) (stale OnComponentBeginOverlap(Collider_Replay) OtherActor)))
      (Variables|/Game/01_Character/Blueprints/BP_FirstPersonGameMode.BP_FirstPersonGameMode_C|SetReplayDiskHIT (Variables|01_Character|GetGM) true)
      (Variables|01_Character|SetPlayer_Hit true))))

(event OnComponentHit(Box)
  (params (HitComponent :type Primitive%20Component%20Object%20Reference) (OtherActor :type Actor%20Object%20Reference) (OtherComp :type Primitive%20Component%20Object%20Reference) (NormalImpulse :type Vector :default "0, 0, 0") (Hit :type Hit%20Result%20Structure%20%28by%20ref%29))
  ;[0.15 0.15 0.15 0.5] SecondCollision
  (Utilities|FlowControl|Sequence
    (:then_0
      (if (Actor|ActorHasTag OtherActor "Simu")
        (Development|PrintString "HAS SIMU")
        (Physics|AddImpulse OtherComp (Variables|Default|GetImpulse) "None" true)))
    (:then_1
      ;;[0.15 0.15 0.15 0.5] SetLocation&NormalHit
      (Variables|02_DiskProperties|SetHitLocation (.location Hit))
      (Variables|02_DiskProperties|SetHitNormal (.normal Hit))
      (if (Actor|ActorHasTag OtherActor "Concrete")
        (Utilities|FlowControl|DoOnce false
          (:Completed
            (CallFunction|ConcreteHit)
            (Utilities|FlowControl|Delay 0.1 :!label _label)
            ;[0.15 0.15 0.15 0.5 32] EXPLOSE SUR UNE SURFACE
            (Actor|DestroyActor)))
        (elif (Actor|ActorHasTag OtherActor "Plastic")
          (CallFunction|RebondScreen)
          (else
            (Utilities|FlowControl|DoOnce false
              (:Completed
                (CallFunction|ConcreteHit)
                (goto _label)))))))))

(event OnComponentBeginOverlap(Collider_Replay)
  (params (OverlappedComponent :type Primitive%20Component%20Object%20Reference) (OtherActor :type Actor%20Object%20Reference) (OtherComp :type Primitive%20Component%20Object%20Reference) (OtherBodyIndex :type Integer) (bFromSweep :type Boolean) (SweepResult :type Hit%20Result%20Structure%20%28by%20ref%29))
  ;[0.1529 0.15 0.5029 0.502] First Collision
  (if (Variables|02_DiskProperties|GetReplayDisc)
    (if (not (== (Components|GetOwner) OtherActor))
      (Variables|/Game/01_Character/Blueprints/BP_FirstPersonGameMode.BP_FirstPersonGameMode_C|SetReplayDiskHIT (Variables|01_Character|GetGM) true)
      (Variables|01_Character|SetPlayer_Hit true))))

(event OnComponentBeginOverlap(PlayerHit_01)
  (params (OverlappedComponent :type Primitive%20Component%20Object%20Reference) (OtherActor :type Actor%20Object%20Reference) (OtherComp :type Primitive%20Component%20Object%20Reference) (OtherBodyIndex :type Integer) (bFromSweep :type Boolean) (SweepResult :type Hit%20Result%20Structure%20%28by%20ref%29))
  (bind _returnvalue (Transformation|GetActorTransform))
  (bind _gm (Variables|01_Character|GetGM))
  ;[0.1529 0.15 0.5029 0.502] First Collision
  (Utilities|FlowControl|Sequence
    (:then_0
      (Variables|02_DiskProperties|SetHitLocation (.Location (Collision|BreakHitResult SweepResult)))
      ;;[0.03434 0.03434 0.1144 0.502] ReplaySystem
      (if (Variables|02_DiskProperties|GetReplayDisc)
        (if (or (== (Variables|01_Character|GetP1) OtherActor) (== (Variables|01_Character|GetP2) OtherActor))
          (if (== (Components|GetOwner) OtherActor)
            _))
        (else
          ;;[0.03434 0.03434 0.1144 0.502] TOUCHE UN JOUEUR
          (if (not (== OtherActor self))
            (|Check_Outcome_2 (Utilities|GetClass self) OtherActor
              (:Mort%20P2
                (Game|SpawnActorfromClass "/Game/01_Character/Blueprints/BP_VisualExplosionP1.BP_VisualExplosionP1_C" _returnvalue "Undefined" "MultiplyWithRoot" 0 false false 0)
                (Variables|/Game/01_Character/Blueprints/BP_FirstPersonGameMode.BP_FirstPersonGameMode_C|SetFakeDisk _gm true)
                (Default|Player2Hit _gm))
              (:Mort%20P1
                (Game|SpawnActorfromClass "/Game/01_Character/Blueprints/BP_VisualExplosionP2.BP_VisualExplosionP2_C" _returnvalue "Undefined" "MultiplyWithRoot" 0 false false 0)
                (Variables|/Game/01_Character/Blueprints/BP_FirstPersonGameMode.BP_FirstPersonGameMode_C|SetFakeDisk _gm true)
                (Default|Player1Hit _gm)))
            (Class|BPIDodgeHit|PlayerDirectHit(Message) (Game|GetGameMode) (Transformation|GetActorLocation))
            (Utilities|DestroyDisc)))))))

(event Custom|Lock%20on
  (params (HommingForce :type Float%20%28double-precision%29))
  (bind _projectilemovement (Variables|Default|GetProjectileMovement))
  ;[0.15 0.15 0.15 0.5] Homing
  (bind _out_homing_target (CallFunction|FindHomingTarget))
  (Variables|/Script/Engine.ProjectileMovementComponent|SetHomingTargetComponent _projectilemovement _out_homing_target)
  (Variables|/Script/Engine.ProjectileMovementComponent|SetbIsHomingProjectile _projectilemovement true)
  (bind _homing (Timeline|Timeline PlayFromStart)
    (:Update
      (Variables|/Script/Engine.ProjectileMovementComponent|SetHomingAccelerationMagnitude _projectilemovement (* (* _homing HommingForce) (Math|Float|SelectFloat 1.5 0.35 (<= (Transformation|GetDistanceTo (Components|GetOwner _out_homing_target)) (Variables|Default|GetDistance))))))))

(event Custom|ConcreteHit
  ;[0.15 0.15 0.15 0.5 32] EXPLOSE SUR UNE SURFACE
  (if (Variables|02_DiskProperties|GetReplayDisc)
    (Utilities|FlowControl|DoOnce false
      (:Completed
        (Game|SpawnActorfromClass "/Game/01_Character/Blueprints/BP_VisualExplosionP1.BP_VisualExplosionP1_C" (Transformation|GetActorTransform) "Undefined" "MultiplyWithRoot" 0 true true 0)
        (Utilities|DestroyDisc :!label _label)))
    (elif (or (== (Variables|01_Character|GetP1) (Utilities|GetClass (stale OnComponentHit(Box) OtherActor))) (== (Variables|01_Character|GetP2) (Utilities|GetClass (stale OnComponentHit(Box) OtherActor))))
      (Class|BPIDodgeHit|PlayerDirectHit(Message) (Game|GetGameMode) (Transformation|GetActorLocation))
      (Variables|01_Character|SetPlayer_Hit false)
      (goto _label)
      (elif (== (Utilities|GetClass self) "/Game/01_Character/Blueprints/00_Character/BP_DiscP1.BP_DiscP1_C")
        (Game|SpawnActorfromClass "/Game/01_Character/Blueprints/BP_Explosion_FromP1.BP_Explosion_FromP1_C" (Math|Transform|MakeTransform (Transformation|GetActorLocation) "0, 0, 0" "1.000000,1.000000,1.000000") "Undefined" "MultiplyWithRoot" 0 true false 0)
        (|SetupDecal :!label _label_2)
        (goto _label)
        (elif (== (Utilities|GetClass self) "/Game/01_Character/Blueprints/00_Character/BP_DiscP2.BP_DiscP2_C")
          (Game|SpawnActorfromClass "/Game/01_Character/Blueprints/BP_Explosion_FromP2.BP_Explosion_FromP2_C" (Math|Transform|MakeTransform (Transformation|GetActorLocation) "0, 0, 0" "1.000000,1.000000,1.000000") "Undefined" "MultiplyWithRoot" 0 true false 0)
          (goto _label_2)
          (elif (== (Utilities|GetClass self) "/Game/01_Character/Blueprints/00_Character/BP_DiscRobot.BP_DiscRobot_C")
            (Game|SpawnActorfromClass "/Game/01_Character/Blueprints/BP_Explosion_FromRobot.BP_Explosion_FromRobot_C" (Math|Transform|MakeTransform (Transformation|GetActorLocation) "0, 0, 0" "1.000000,1.000000,1.000000") "Undefined" "MultiplyWithRoot" 0 true false 0)))))))

(event Custom|RebondScreen
  (bind _hitlocation (Variables|02_DiskProperties|GetHitLocation))
  (bind _startpos (Variables|02_DiskProperties|GetStartPos))
  (bind _hitnormal (Variables|02_DiskProperties|GetHitNormal))
  (bind _returnvalue (Math|Vector|GetUnitDirection(Vector) _startpos _hitlocation))
  (bind _returnvalue_2 (Math|Vector|MirrorVectorbyNormal _returnvalue _hitnormal))
  ;[0.15 0.15 0.15 0.5 32] Bounce
  (bind _result (Math|Integer|IncrementInt (Variables|02_DiskProperties|GetBounceNB))
    (:%20%20
      (Variables|02_DiskProperties|SetBounceNB _result)
      ;;[1 0 0.4024 0.5 24] BounceSound
      (Audio|SpawnSound2D "/Game/05_SONS/Disque/DODGEHIT_SD_rebond_disque_V01.DODGEHIT_SD_rebond_disque_V01" 2.0 1.0 0.8 0)
      ;;[0.15 0.15 0.15 0.5] SetupHommingNiagara
      (CallFunction|Lockon 1.5)
      (Variables|02_DiskProperties|SetPosBounce _returnvalue_2)
      (|SetupNiagara (Variables|02_DiskProperties|GetHitLocation) _returnvalue_2 (Math|Conversions|RotationFromXVector _hitnormal)))))

(event EventBeginPlay
  ;[1 0.15 0.15 0.5 32] Begin Play
  (|NodesBeginPlay
    (:execute2
      (CallFunction|Lockon 1.0)
      (if (not (Variables|02_DiskProperties|GetReplayDisc))
        ;;[1 0 0.4969 0.502] Start
        (Audio|SpawnSound2D "/Game/05_SONS/Disque/DODGEHIT_SD_disk_throw_A_V04.DODGEHIT_SD_disk_throw_A_V04" 0.85 1.0 0.15 0)
        (if (== (Math|Random|RandomIntegerinRange 0 6) 0)
          (Utilities|FlowControl|Delay 0.3)
          ;;[1 0 0.4969 0.502] SOUND
          (Audio|PlaySound2D "/Game/05_SONS/Disque/OLD/CrowdGasp.CrowdGasp" 0.4 1.2 0.2 0 0))))))

(event EventPlayerDirectHit
  (params (DirectHitLocation :type Vector :default "0, 0, 0"))
  ;[0.15 0.15 0.15 0.5 32] EXPLOSE SUR UNE SURFACE
  (if (Variables|02_DiskProperties|GetReplayDisc)
    (Utilities|FlowControl|DoOnce false
      (:Completed
        (Game|SpawnActorfromClass "/Game/01_Character/Blueprints/BP_VisualExplosionP1.BP_VisualExplosionP1_C" (Transformation|GetActorTransform) "Undefined" "MultiplyWithRoot" 0 true true 0)
        (Utilities|DestroyDisc :!label _label)))
    (elif (or (== (Variables|01_Character|GetP1) (Utilities|GetClass (stale OnComponentHit(Box) OtherActor))) (== (Variables|01_Character|GetP2) (Utilities|GetClass (stale OnComponentHit(Box) OtherActor))))
      (Class|BPIDodgeHit|PlayerDirectHit(Message) (Game|GetGameMode) (Transformation|GetActorLocation))
      (Variables|01_Character|SetPlayer_Hit false)
      (goto _label)
      (elif (== (Utilities|GetClass self) "/Game/01_Character/Blueprints/00_Character/BP_DiscP1.BP_DiscP1_C")
        (Game|SpawnActorfromClass "/Game/01_Character/Blueprints/BP_Explosion_FromP1.BP_Explosion_FromP1_C" (Math|Transform|MakeTransform (Transformation|GetActorLocation) "0, 0, 0" "1.000000,1.000000,1.000000") "Undefined" "MultiplyWithRoot" 0 true false 0)
        (|SetupDecal :!label _label_2)
        (goto _label)
        (elif (== (Utilities|GetClass self) "/Game/01_Character/Blueprints/00_Character/BP_DiscP2.BP_DiscP2_C")
          (Game|SpawnActorfromClass "/Game/01_Character/Blueprints/BP_Explosion_FromP2.BP_Explosion_FromP2_C" (Math|Transform|MakeTransform (Transformation|GetActorLocation) "0, 0, 0" "1.000000,1.000000,1.000000") "Undefined" "MultiplyWithRoot" 0 true false 0)
          (goto _label_2)
          (elif (== (Utilities|GetClass self) "/Game/01_Character/Blueprints/00_Character/BP_DiscRobot.BP_DiscRobot_C")
            (Game|SpawnActorfromClass "/Game/01_Character/Blueprints/BP_Explosion_FromRobot.BP_Explosion_FromRobot_C" (Math|Transform|MakeTransform (Transformation|GetActorLocation) "0, 0, 0" "1.000000,1.000000,1.000000") "Undefined" "MultiplyWithRoot" 0 true false 0)))))))

(event EventTick
  (params (DeltaSeconds :type Float%20%28single-precision%29))
  (bind _projectilemovement (Variables|Default|GetProjectileMovement))
  ;[0.15 0.15 0.15 0.5] Speed Disc
  (Utilities|CustomBranch
    (:true
      (Game|Components|ProjectileMovement|SetVelocityinLocalSpace _projectilemovement "0, 0, 0"))
    (:false
      (Game|Components|ProjectileMovement|SetVelocityinLocalSpace _projectilemovement (Variables|02_DiskProperties|GetSpeedDiscManager)))))

(fn ConstructionScript)

(fn FindHomingTarget
  (bind _outactors (Actor|GetAllActorsOfClasswithTag "/Script/Engine.Actor" "player"))
  (for _array_element _outactors
    (LocalVariables|SetActorFind _array_element)
    (if (< (Math|Vector|VectorLength (- (Transformation|GetActorLocation _array_element) (Transformation|GetActorLocation))) (LocalVariables|Getcloset%20distance))
      (LocalVariables|Setcloset%20distance (Math|Vector|VectorLength (- (Transformation|GetActorLocation _array_element) (Transformation|GetActorLocation))))
      (Utilities|FlowControl|Sequence
        (:then_0
          (Variables|Default|SetDistance 1.5e+03)
          (if (Actor|ActorHasTag "DiscP1")
            (LocalVariables|SetHomingTarget (Variables|Default|GetTargetHommingP2))
            (bind _returnvalue (UserInterface|CreateWidget "/Game/03_UI/01_INGame/02_Damage_Close/Widget_P2_Target.Widget_P2_Target_C"))
            (bind _output_get (Variables|04_Widget|SetWidgetToDestroy _returnvalue))
            (UserInterface|Viewport|AddtoViewport _output_get 0)
            (else
              (LocalVariables|SetHomingTarget (Variables|Default|GetTargetHommingP1))
              (bind _returnvalue_2 (UserInterface|CreateWidget "/Game/03_UI/01_INGame/02_Damage_Close/Widget_P1_Target.Widget_P1_Target_C"))
              (bind _output_get_2 (Variables|04_Widget|SetWidgetToDestroy _returnvalue_2))
              (UserInterface|Viewport|AddtoViewport _output_get_2 0)))))))
  (Utilities|FlowControl|Sequence
    (:then_0
      (return (Actor|GetComponentbyClass (LocalVariables|GetHomingTarget) "/Script/Engine.SceneComponent")))
    (:then_1
      (if (or (!= (LocalVariables|GetActorFind) (Variables|01_Character|GetP1)) (!= (LocalVariables|GetActorFind) (Variables|01_Character|GetP2)))
        (Development|PrintString (Utilities|GetDisplayName (LocalVariables|GetActorFind)))
        (Variables|Default|SetDistance 5e+02)
        (LocalVariables|SetHomingTarget (LocalVariables|GetActorFind))))))