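; BP_Character_P2 is the Player 2 variant of a parent character Blueprint.
; It clears the P1P2 flag on BeginPlay and loads Player 2's saved gamepad sensitivity from the save game, which LoadSaveVariables can also re-trigger.
; The pause input calls Paused for Player 2 on all P2 characters, provided Player 1 has not paused and the game mode's pause menu is closed.
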(event Custom|LoadSaveVariables
  (params (SlotName :type String))
  (bind _slot_name (Variables|Default|GetSlot%20Name))
  (bind _returnvalue (SaveGame|DoesSaveGameExist _slot_name))
  (if _returnvalue
    (bind _returnvalue_2 (SaveGame|LoadGamefromSlot _slot_name))
    (bind _asbp_save_game_variables (Utilities|Casting|CastToBP_SaveGameVariables _returnvalue_2))
    (Variables|Default|SetGamepad%20Sensivity (Variables|/Game/BP_SaveGameVariables.BP_SaveGameVariables_C|GetSaved_Player_2_Sens _asbp_save_game_variables))))

(event Input|EnhancedActionEvents|EnhancedInputActionIA_PausedPlayer
  (params (ActionValue :type Boolean) (ElapsedSeconds :type Float%20%28double-precision%29) (TriggeredSeconds :type Float%20%28double-precision%29) (InputAction :type Input%20Action%20Object%20Reference :default "/Game/01_Character/Input/Actions/IA_PausedPlayer.IA_PausedPlayer"))
  (:Started
    (if (not (Variables|Default|GetPausedP1))
      (if (not (Variables|/Game/01_Character/Blueprints/BP_FirstPersonGameMode.BP_FirstPersonGameMode_C|GetMenuPause%20Open (Variables|Default|GetGM)))
        (bind _outactors (Actor|GetAllActorsOfClass "BP_Character_P2_C"))
        (for _array_element _outactors
          (Default|Paused _array_element false true))))))

(event EventBeginPlay
  (bind _slot_name (Variables|Default|GetSlot%20Name))
  (Utilities|FlowControl|Sequence
    (:then_0
      (|CallParentFunction)
      (Variables|Default|SetP1/P2 false))
    (:then_1
      (bind _returnvalue (SaveGame|DoesSaveGameExist _slot_name))
      (if _returnvalue
        (bind _returnvalue_2 (SaveGame|LoadGamefromSlot _slot_name))
        (bind _asbp_save_game_variables (Utilities|Casting|CastToBP_SaveGameVariables _returnvalue_2))
        (Variables|Default|SetGamepad%20Sensivity (Variables|/Game/BP_SaveGameVariables.BP_SaveGameVariables_C|GetSaved_Player_2_Sens _asbp_save_game_variables))))))

(event EventTick
  (params (DeltaSeconds :type Float%20%28single-precision%29))
  (|CallParentFunction DeltaSeconds))

(fn ConstructionScript
  (|CallParentFunction))