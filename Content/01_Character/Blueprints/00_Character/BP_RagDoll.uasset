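; Ragdoll actor that simulates physics on spawn, leaves splash decals, then dissolves and destroys itself.
; BeginPlay picks a cloth material by player side and makes dynamic instances for four material slots.
; Each slot's branch runs into a shared chain that spawns a random decal and waits on a delay.
; A timeline then raises Erosion on all four materials, and finishing resets MPC_RagDoll's Erosion and spawns another decal.
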(event EventBeginPlay
  (bind _skeletalmesh (Variables|Default|GetSkeletalMesh))
  (bind _skeletalmesh_2 (Variables|Default|GetSkeletalMesh))
  (Rendering|Material|SetMaterial (Variables|Default|GetSkeletalMesh) 2 (select (Variables|Default|GetP1/P2) "/Game/03_VFX/02_Material/04_Chara/MI_CLOTH_Recolor_VFX.MI_CLOTH_Recolor_VFX" "/Game/03_VFX/02_Material/04_Chara/MI_CLOTH_VFX.MI_CLOTH_VFX"))
  (Physics|SetSimulatePhysics (Variables|Default|GetSkeletalMesh) true)
  (Utilities|FlowControl|Sequence
    (:then_0
      ;[0.15 0.15 0.15 0.5] ConfigureDynamicMaterial
      (bind _dynamicmaterial (CallFunction|SetDynamicMaterial _skeletalmesh))
      (bind _output_get (Variables|DM|SetDM_Mat01 _dynamicmaterial))
      (Rendering|Material|SetMaterial _skeletalmesh_2 0 _output_get))
    (:then_1
      (bind _dynamicmaterial_2 (CallFunction|SetDynamicMaterial _skeletalmesh 1))
      (bind _output_get_2 (Variables|DM|SetDM_Mat02 _dynamicmaterial_2))
      (Rendering|Material|SetMaterial _skeletalmesh_2 1 _output_get_2))
    (:then_2
      (bind _dynamicmaterial_3 (CallFunction|SetDynamicMaterial _skeletalmesh 2))
      (bind _output_get_3 (Variables|DM|SetDM_Mat03 _dynamicmaterial_3))
      (Rendering|Material|SetMaterial _skeletalmesh_2 2 _output_get_3))
    (:then_3
      (bind _dynamicmaterial_4 (CallFunction|SetDynamicMaterial _skeletalmesh 3))
      (bind _output_get_4 (Variables|DM|SetDM_Mat04 _dynamicmaterial_4))
      (Rendering|Material|SetMaterial _skeletalmesh_2 3 _output_get_4)))
  (Rendering|Decal|SpawnDecalatLocation (Utilities|Select :Index (Math|Random|RandomInteger 5) :Option%200 "/Game/03_VFX/02_Material/02_Enviro/Mi_SplashDecal.Mi_SplashDecal" :Option%201 "/Game/03_VFX/02_Material/02_Enviro/Mi_SplashDecal02.Mi_SplashDecal02" :Option%202 "/Game/03_VFX/02_Material/02_Enviro/Mi_SplashDecal03.Mi_SplashDecal03" :Option%203 "/Game/03_VFX/02_Material/02_Enviro/Mi_SplashDecal04.Mi_SplashDecal04") (Math|Vector|MakeVector 2.5e+02 2.5e+02 2.5e+02) (Transformation|GetWorldLocation (Variables|Default|GetSkeletalMesh)) (Math|Random|RandomRotator true) (Math|Random|RandomFloatinRange 5.0 15.0))
  (Utilities|FlowControl|Delay 7.5)
  (bind _lerp_dissolution (Timeline|T_TIME PlayFromStart)
    (:Update
      (Rendering|Material|SetScalarParameterValue (Variables|DM|GetDM_Mat01) "Erosion" (Math|Float|Lerp 0.0 1.0 _lerp_dissolution) :!class /Script/Engine.MaterialInstanceDynamic)
      (Rendering|Material|SetScalarParameterValue (Variables|DM|GetDM_Mat02) "Erosion" (Math|Float|Lerp 0.0 1.0 _lerp_dissolution) :!class /Script/Engine.MaterialInstanceDynamic)
      (Rendering|Material|SetScalarParameterValue (Variables|DM|GetDM_Mat03) "Erosion" (Math|Float|Lerp 0.0 1.0 _lerp_dissolution) :!class /Script/Engine.MaterialInstanceDynamic)
      (Rendering|Material|SetScalarParameterValue (Variables|DM|GetDM_Mat04) "Erosion" (Math|Float|Lerp 0.0 1.0 _lerp_dissolution) :!class /Script/Engine.MaterialInstanceDynamic))
    (:Finished
      (Rendering|Material|SetScalarParameterValue "/Game/03_VFX/02_Material/00_Master/02_MPC/MPC_RagDoll.MPC_RagDoll" "Erosion" 0.0 :!class /Script/Engine.KismetMaterialLibrary)
      (Rendering|Decal|SpawnDecalatLocation (Utilities|Select :Index (Math|Random|RandomInteger 5) :Option%200 "/Game/03_VFX/02_Material/02_Enviro/Mi_SplashDecal.Mi_SplashDecal" :Option%201 "/Game/03_VFX/02_Material/02_Enviro/Mi_SplashDecal02.Mi_SplashDecal02" :Option%202 "/Game/03_VFX/02_Material/02_Enviro/Mi_SplashDecal03.Mi_SplashDecal03" :Option%203 "/Game/03_VFX/02_Material/02_Enviro/Mi_SplashDecal04.Mi_SplashDecal04") (Math|Vector|MakeVector 2.5e+02 2.5e+02 2.5e+02) (Transformation|GetWorldLocation (Variables|Default|GetSkeletalMesh)) (Math|Random|RandomRotator true) (Math|Random|RandomFloatinRange 5.0 15.0))
      (Actor|DestroyActor))))

(fn ConstructionScript)

(fn SetDynamicMaterial
  (params (SkeletalMesh :type Primitive%20Component%20Object%20Reference) (MatIndex :type Integer))
  (bind _returnvalue (Rendering|Material|CreateDynamicMaterialInstance (Rendering|Material|GetMaterial SkeletalMesh MatIndex) "None" "None" :!class /Script/Engine.KismetMaterialLibrary))
  (return _returnvalue))