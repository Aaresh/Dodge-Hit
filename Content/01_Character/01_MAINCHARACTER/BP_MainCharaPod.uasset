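; BP_MainCharaPod is the main character's pod, whose fluid simulation and fluid collider turn on or off based on camera view and start state.
; On BeginPlay and each Update call, camera view 2 restarts the simulation and shows both components with their children.
; In any other view, both are hidden unless the started flag is set.
; Update stores the started flag, then reruns the same check.
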(event Custom|Update
  (params (CamV :type Integer) (STARTED :type Boolean))
  (Variables|Default|SetSTARTED STARTED)
  (if (== CamV 2)
    (Components|Timeline|PlayfromStart (Variables|Default|GetFluidSimulation))
    (Rendering|SetVisibility (Variables|Default|GetFluidCollider) true true)
    (elif (not STARTED)
      (Rendering|SetVisibility (Variables|Default|GetFluidSimulation) false false))))

(event EventBeginPlay
  (if (== (stale Custom|Update CamV) 2)
    (Components|Timeline|PlayfromStart (Variables|Default|GetFluidSimulation))
    (Rendering|SetVisibility (Variables|Default|GetFluidCollider) true true)
    (elif (not (stale Custom|Update STARTED))
      (Rendering|SetVisibility (Variables|Default|GetFluidSimulation) false false))))

(fn ConstructionScript)