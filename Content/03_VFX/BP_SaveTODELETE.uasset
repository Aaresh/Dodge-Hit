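; Scratch Blueprint, marked for deletion by its name, that holds hold-to-skip input logic for cinematics.
; Separate gamepad and keyboard Enhanced Input actions pass hold time to the AnimSkip radial bars while triggered and call the matching cancel on completion.
; Both paths set CinematicSkip by comparing hold time to TimeToSkip, but the branch that follows does nothing.
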(event Input|EnhancedActionEvents|EnhancedInputActionIA_SkipCinematicsKeyBoard
  (params (ActionValue :type Boolean) (ElapsedSeconds :type Float%20%28double-precision%29) (TriggeredSeconds :type Float%20%28double-precision%29) (InputAction :type Input%20Action%20Object%20Reference :default "/Game/01_Character/Input/Actions/IA_SkipCinematicsKeyBoard.IA_SkipCinematicsKeyBoard"))
  (bind _animskip (Variables|Default|GetAnimSkip))
  (:Triggered
    (Default|SetRadialKeyBoard _animskip TriggeredSeconds)
    (Default|RadialBarKeyBoard _animskip)
    (bind _output_get (Variables|Default|SetCinematicSkip (or (>= (stale Input|EnhancedActionEvents|EnhancedInputActionIA_SkipCinematicsGamePad TriggeredSeconds) (Variables|Default|GetTimeToSkip)) (>= TriggeredSeconds (Variables|Default|GetTimeToSkip)))))
    (if _output_get
      _))
  (:Completed
    (Default|CancelledKeyboard (Variables|Default|GetAnimSkip))))

(event Input|EnhancedActionEvents|EnhancedInputActionIA_SkipCinematicsGamePad
  (params (ActionValue :type Boolean) (ElapsedSeconds :type Float%20%28double-precision%29) (TriggeredSeconds :type Float%20%28double-precision%29) (InputAction :type Input%20Action%20Object%20Reference :default "/Game/01_Character/Input/Actions/IA_SkipCinematicsGamePad.IA_SkipCinematicsGamePad"))
  (bind _animskip (Variables|Default|GetAnimSkip))
  (:Triggered
    (Default|SetRadialGamePad _animskip TriggeredSeconds)
    (Default|RadialBarController _animskip)
    (bind _output_get (Variables|Default|SetCinematicSkip (or (>= TriggeredSeconds (Variables|Default|GetTimeToSkip)) (>= (stale Input|EnhancedActionEvents|EnhancedInputActionIA_SkipCinematicsKeyBoard TriggeredSeconds) (Variables|Default|GetTimeToSkip)))))
    (if _output_get
      _))
  (:Completed
    (Default|CancelledController (Variables|Default|GetAnimSkip))))

(fn ConstructionScript)