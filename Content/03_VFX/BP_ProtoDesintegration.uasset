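; Prototype VFX Blueprint for a staggered disintegration of a main mesh and red, green and blue fiber meshes.
; Each mesh gets a dynamic material instance, with timelines animating its scalar parameters.
; After an initial delay, the main mesh starts dissolving, then each fiber follows at increasing offsets through parallel Sequence branches.
; No event triggers this chain, so it never runs as wired, and stray parameter-reset nodes are also unconnected.
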(fn ConstructionScript)