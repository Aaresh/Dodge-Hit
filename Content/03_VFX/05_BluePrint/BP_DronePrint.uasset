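; Drone VFX actor that briefly fires two spawn-band Niagara beams, then flies its Drone component along a spline.
; BeginPlay sets the beam ends to ankle and hand socket locations read from a Material Parameter Collection, then starts the sequence.
; A fast looping timer advances the drone with increasing speed until the last spline point; Activate resets and replays it.
; A Timeline driving a material "Resolve" parameter is present but never runs.
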(event Custom|Start
  (bind _drone (Variables|Default|GetDrone))
  (bind _spline (Variables|Default|GetSpline))
  (bind _output_get (Variables|Default|SetTime (+ (Variables|Default|GetTime) 1e-05)))
  (bind _output_get_2 (Variables|Default|SetDistanceAlongSpline (+ (* _output_get (Variables|Default|GetSpeedAlongSpline)) (Variables|Default|GetDistanceAlongSpline))))
  (Transformation|SetRelativeTransform _drone (Math|Transform|MakeTransform (.location (Spline|GetTransformatDistanceAlongSpline _spline _output_get_2 "Local" false)) (Math|Rotator|CombineRotators (.rotation (Spline|GetTransformatDistanceAlongSpline _spline _output_get_2 "Local" false)) "0.000000,-90.000000,0.000000") (Variables|/Script/Engine.SceneComponent|GetRelativeScale3D _drone)) false false)
  (if (Utilities|Operators|EqualEqual (.location (Spline|GetTransformatDistanceAlongSpline _spline _output_get_2 "Local" false)) (.location (Spline|GetTransformatSplinePoint _spline (- (Spline|GetNumberOfSplinePoints _spline) 1) "Local" false)) 0.0)
    (Utilities|Time|ClearandInvalidateTimerbyHandle (stale Custom|Activate _returnvalue))))

(event Custom|Activate
  (Transformation|SetRelativeTransform (Variables|Default|GetDrone) (Variables|Default|GetStartTransform) false false)
  (Variables|Default|SetTime 0.0)
  (Variables|Default|SetDistanceAlongSpline 0.0)
  (Components|Activation|Activate (Variables|Default|GetNS_SpawnBand) false)
  (Utilities|FlowControl|Delay 0.5)
  (bind _returnvalue (Utilities|Time|SetTimerbyEvent (delegate Custom|Start) 0.001 true))
  (Components|Activation|Deactivate (Variables|Default|GetNS_SpawnBand)))

(event EventBeginPlay
  ;[0.15 0.15 0.15 0.5] Ankle
  (bind _returnvalue (Rendering|Material|GetVectorParameterValue "/Game/03_VFX/02_Material/00_Master/02_MPC/MPC_TransferSocketLocation.MPC_TransferSocketLocation" "AnkleSocket_Location" :!class /Script/Engine.KismetMaterialLibrary))
  (Effects|Components|ParticleSystem|SetVectorParameter (Variables|Default|GetNS_SpawnBand) "BeamEnd" (Math|Vector|MakeVector (.R (Math|Color|BreakColor _returnvalue)) (.G (Math|Color|BreakColor _returnvalue)) (.B (Math|Color|BreakColor _returnvalue))))
  ;[0.15 0.15 0.15 0.5] Hand
  (bind _returnvalue_2 (Rendering|Material|GetVectorParameterValue "/Game/03_VFX/02_Material/00_Master/02_MPC/MPC_TransferSocketLocation.MPC_TransferSocketLocation" "HandSocket_Location" :!class /Script/Engine.KismetMaterialLibrary))
  (Development|PrintString (Utilities|String|ToString(Vector) (Math|Vector|MakeVector (.R (Math|Color|BreakColor _returnvalue_2)) (.G (Math|Color|BreakColor _returnvalue_2)) (.B (Math|Color|BreakColor _returnvalue_2)))))
  (Effects|Components|ParticleSystem|SetVectorParameter (Variables|Default|GetNS_SpawnBand1) "BeamEnd" (Math|Vector|MakeVector (.R (Math|Color|BreakColor _returnvalue_2)) (.G (Math|Color|BreakColor _returnvalue_2)) (.B (Math|Color|BreakColor _returnvalue_2))))
  (Variables|Default|SetStartTransform (Transformation|GetRelativeTransform (Variables|Default|GetDrone)))
  (Utilities|FlowControl|Delay 0.2)
  (Components|Activation|Activate (Variables|Default|GetNS_SpawnBand) false)
  (Utilities|FlowControl|Delay 0.5)
  (bind _returnvalue_3 (Utilities|Time|SetTimerbyEvent (delegate Custom|Start) 0.001 true))
  (Components|Activation|Deactivate (Variables|Default|GetNS_SpawnBand)))

(fn ConstructionScript)

(fn SetDynamicMaterial
  (params (MatIndex :type Integer) (NewParam :type Skeletal%20Mesh%20Component%20Object%20Reference))
  (bind _returnvalue (Rendering|Material|CreateDynamicMaterialInstance (Rendering|Material|GetMaterial NewParam MatIndex) "None" "None" :!class /Script/Engine.KismetMaterialLibrary))
  (return _returnvalue))