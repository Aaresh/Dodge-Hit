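; VFX manager for a drone "print" effect, tied to the P1 or P2 character, that moves a drone along a spline with spawn beams.
; BeginPlay aims three Niagara bands at that player's ankle, hand and body locations, read once from a Material Parameter Collection.
; It, or Activate on replay, fires the bands briefly, then a looping timer accelerates the drone to the spline's end.
; A material "Resolve" timeline exists but is never run.
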(event Custom|Start
  (bind _drone (Variables|Default|GetDrone))
  (bind _spline (Variables|Default|GetSpline))
  (bind _output_get (Variables|Default|SetTime (+ (Variables|Default|GetTime) 1e-05)))
  (bind _output_get_2 (Variables|Default|SetDistanceAlongSpline (+ (* _output_get (Variables|Default|GetSpeedAlongSpline)) (Variables|Default|GetDistanceAlongSpline))))
  (Transformation|SetRelativeTransform _drone (Math|Transform|MakeTransform (.location (Spline|GetTransformatDistanceAlongSpline _spline _output_get_2 "Local" false)) (Math|Rotator|CombineRotators (.rotation (Spline|GetTransformatDistanceAlongSpline _spline _output_get_2 "Local" false)) "0.000000,-90.000000,0.000000") (Variables|/Script/Engine.SceneComponent|GetRelativeScale3D _drone)) false false)
  (if (Utilities|Operators|EqualEqual (.location (Spline|GetTransformatDistanceAlongSpline _spline _output_get_2 "Local" false)) (.location (Spline|GetTransformatSplinePoint _spline (- (Spline|GetNumberOfSplinePoints _spline) 1) "Local" false)) 0.0)
    (Utilities|Time|ClearandInvalidateTimerbyHandle (stale Custom|Activate _returnvalue))))

(event Custom|Activate
  (Transformation|SetRelativeTransform (Variables|Default|GetDrone) (Variables|Default|GetStartTransform) false false)
  (Variables|Default|SetTime 0.0)
  (Variables|Default|SetDistanceAlongSpline 0.0)
  (Components|Activation|Activate (Variables|Default|GetNS_SpawnBand) false)
  (Utilities|FlowControl|Delay 1.0)
  (bind _returnvalue (Utilities|Time|SetTimerbyEvent (delegate Custom|Start) 0.001 true))
  (Components|Activation|Deactivate (Variables|Default|GetNS_SpawnBand)))

(event EventBeginPlay
  (Utilities|FlowControl|Delay 0.2)
  (if (Variables|Default|GetP1/P2)
    (bind _returnvalue (Actor|GetActorOfClass "/Game/01_Character/Blueprints/00_Character/BP_Character_P1.BP_Character_P1_C"))
    (Actor|SetOwner _returnvalue)
    ;[0.15 0.15 0.15 0.5] P1
    ;;[0.15 0.15 0.15 0.5] Ankle
    (bind _returnvalue_2 (Rendering|Material|GetVectorParameterValue "/Game/03_VFX/02_Material/00_Master/02_MPC/MPC_TransferSocketLocation.MPC_TransferSocketLocation" "AnkleSocket_LocationP1" :!class /Script/Engine.KismetMaterialLibrary))
    (Effects|Components|ParticleSystem|SetVectorParameter (Variables|Default|GetNS_SpawnBand) "BeamEnd" (Math|Vector|MakeVector (.R (Math|Color|BreakColor _returnvalue_2)) (.G (Math|Color|BreakColor _returnvalue_2)) (.B (Math|Color|BreakColor _returnvalue_2))))
    ;;[0.15 0.15 0.15 0.5] Hand
    (bind _returnvalue_3 (Rendering|Material|GetVectorParameterValue "/Game/03_VFX/02_Material/00_Master/02_MPC/MPC_TransferSocketLocation.MPC_TransferSocketLocation" "HandSocket_LocationP1" :!class /Script/Engine.KismetMaterialLibrary))
    (Effects|Components|ParticleSystem|SetVectorParameter (Variables|Default|GetNS_SpawnBand1) "BeamEnd" (Math|Vector|MakeVector (.R (Math|Color|BreakColor _returnvalue_3)) (.G (Math|Color|BreakColor _returnvalue_3)) (.B (Math|Color|BreakColor _returnvalue_3))))
    ;;[0.15 0.15 0.15 0.5] Hand
    (bind _returnvalue_4 (Rendering|Material|GetVectorParameterValue "/Game/03_VFX/02_Material/00_Master/02_MPC/MPC_TransferSocketLocation.MPC_TransferSocketLocation" "BodySocket_LocationP1" :!class /Script/Engine.KismetMaterialLibrary))
    (Effects|Components|ParticleSystem|SetVectorParameter (Variables|Default|GetNS_SpawnBand2) "BeamEnd" (Math|Vector|MakeVector (.R (Math|Color|BreakColor _returnvalue_4)) (.G (Math|Color|BreakColor _returnvalue_4)) (.B (Math|Color|BreakColor _returnvalue_4))))
    (else
      (bind _returnvalue_5 (Actor|GetActorOfClass "/Game/01_Character/Blueprints/00_Character/BP_Character_P2.BP_Character_P2_C"))
      (Actor|SetOwner _returnvalue_5)
      ;[0.15 0.15 0.15 0.5] P2
      ;;[0.15 0.15 0.15 0.5] Ankle
      (bind _returnvalue_6 (Rendering|Material|GetVectorParameterValue "/Game/03_VFX/02_Material/00_Master/02_MPC/MPC_TransferSocketLocation.MPC_TransferSocketLocation" "AnkleSocket_LocationP2" :!class /Script/Engine.KismetMaterialLibrary))
      (Effects|Components|ParticleSystem|SetVectorParameter (Variables|Default|GetNS_SpawnBand) "BeamEnd" (Math|Vector|MakeVector (.R (Math|Color|BreakColor _returnvalue_6)) (.G (Math|Color|BreakColor _returnvalue_6)) (.B (Math|Color|BreakColor _returnvalue_6))))
      ;;[0.15 0.15 0.15 0.5] Hand
      (bind _returnvalue_7 (Rendering|Material|GetVectorParameterValue "/Game/03_VFX/02_Material/00_Master/02_MPC/MPC_TransferSocketLocation.MPC_TransferSocketLocation" "HandSocket_LocationP2" :!class /Script/Engine.KismetMaterialLibrary))
      (Effects|Components|ParticleSystem|SetVectorParameter (Variables|Default|GetNS_SpawnBand1) "BeamEnd" (Math|Vector|MakeVector (.R (Math|Color|BreakColor _returnvalue_7)) (.G (Math|Color|BreakColor _returnvalue_7)) (.B (Math|Color|BreakColor _returnvalue_7))))
      ;;[0.15 0.15 0.15 0.5] Hand
      (bind _returnvalue_8 (Rendering|Material|GetVectorParameterValue "/Game/03_VFX/02_Material/00_Master/02_MPC/MPC_TransferSocketLocation.MPC_TransferSocketLocation" "BodySocket_LocationP2" :!class /Script/Engine.KismetMaterialLibrary))
      (Effects|Components|ParticleSystem|SetVectorParameter (Variables|Default|GetNS_SpawnBand2) "BeamEnd" (Math|Vector|MakeVector (.R (Math|Color|BreakColor _returnvalue_8)) (.G (Math|Color|BreakColor _returnvalue_8)) (.B (Math|Color|BreakColor _returnvalue_8))))))
  (Variables|Default|SetStartTransform (Transformation|GetRelativeTransform (Variables|Default|GetDrone)))
  (Utilities|FlowControl|Delay 0.2)
  (Components|Activation|Activate (Variables|Default|GetNS_SpawnBand) false)
  (Utilities|FlowControl|Delay 1.0)
  (bind _returnvalue_9 (Utilities|Time|SetTimerbyEvent (delegate Custom|Start) 0.001 true))
  (Components|Activation|Deactivate (Variables|Default|GetNS_SpawnBand)))

(fn ConstructionScript)

(fn SetDynamicMaterial
  (params (MatIndex :type Integer) (NewParam :type Skeletal%20Mesh%20Component%20Object%20Reference))
  (bind _returnvalue (Rendering|Material|CreateDynamicMaterialInstance (Rendering|Material|GetMaterial NewParam MatIndex) "None" "None" :!class /Script/Engine.KismetMaterialLibrary))
  (return _returnvalue))