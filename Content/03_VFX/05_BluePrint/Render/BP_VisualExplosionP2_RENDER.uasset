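; Explosion decal actor for VFX, named as the render variant of VisualExplosionP2.
; On BeginPlay a timeline drives the decal color's alpha through an intensity track.
; When the timeline finishes, the decal fades out after a short delay and destroys its owning actor.
; Random size-vector and actor-location nodes are left unconnected, so the graph applies no size variation.
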(event EventBeginPlay
  (Variables|Default|SetDecalComponent (Variables|Default|GetDecal))
  (Utilities|FlowControl|Sequence
    (:then_1
      (bind _intensity (Timeline|Timeline_0 PlayFromStart)
        (:Update
          (Rendering|Components|Decal|SetDecalColor (Variables|Default|GetDecalComponent) (Utilities|Struct|MakeLinearColor 0.0 0.0 0.0 _intensity)))
        (:Finished
          (Rendering|Components|Decal|SetFadeOut (Variables|Default|GetDecalComponent) 0.5 2.0 true))))))

(fn ConstructionScript)