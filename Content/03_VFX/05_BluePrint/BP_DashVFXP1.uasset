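; BP_DashVFXP1 is a short-lived posed-mesh copy of a character, apparently serving as player one's dash afterimage.
; On BeginPlay it writes the player color to MPC_Slide, takes the first BP_Character_P1 as owner and copies the supplied skeletal component's pose onto its PoseableMesh.
; With a valid source component, it destroys itself after a brief delay.
; The emissive, desaturation and fade timeline and the dynamic material creation are disconnected and never run.
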(event EventBeginPlay
  (Rendering|Material|SetVectorParameterValue "/Game/03_VFX/02_Material/00_Master/02_MPC/MPC_Slide.MPC_Slide" "Player_Color" (Variables|Default|GetColorPlayer) :!class /Script/Engine.KismetMaterialLibrary)
  (Utilities|FlowControl|DoOnce false
    (:Completed
      (bind _outactors (Actor|GetAllActorsOfClass "/Game/01_Character/Blueprints/00_Character/BP_Character_P1.BP_Character_P1_C"))
      (Actor|SetOwner (Utilities|Array|Get(acopy) _outactors))
      (bind _in_component_to_copy (Variables|Default|GetIn%20Component%20to%20Copy)
        (:then
          (Class|PoseableMeshComponent|CopyPosefromSkeletalComponent (Variables|Default|GetPoseableMesh) _in_component_to_copy)
          (Utilities|FlowControl|Delay 0.5)
          (Actor|DestroyActor))
        (:else)))))

(fn ConstructionScript)