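; BP_DeathP2 is a death VFX actor that leaves a fading posed copy of a character, then destroys itself.
; On BeginPlay it pushes the player color to MPC_Slide, sets the first BP_Character_P1 as owner, and copies the supplied skeletal pose onto its PoseableMesh.
; A timeline then drives emissive, desaturation and fade through that shared parameter collection; the dynamic material instance nodes are never run.
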(event EventBeginPlay
  (Rendering|Material|SetVectorParameterValue "/Game/03_VFX/02_Material/00_Master/02_MPC/MPC_Slide.MPC_Slide" "Player_Color" (Variables|Default|GetColorPlayer) :!class /Script/Engine.KismetMaterialLibrary)
  (Utilities|FlowControl|DoOnce false
    (:Completed
      (bind _outactors (Actor|GetAllActorsOfClass "/Game/01_Character/Blueprints/00_Character/BP_Character_P1.BP_Character_P1_C"))
      (Actor|SetOwner (Utilities|Array|Get(acopy) _outactors))
      (bind _in_component_to_copy (Variables|Default|GetIn%20Component%20to%20Copy)
        (:then
          (Class|PoseableMeshComponent|CopyPosefromSkeletalComponent (Variables|Default|GetPoseableMesh) _in_component_to_copy)
          (bind (_direction _emissive _desaturation _fade) (Timeline|Timeline PlayFromStart)
            (:Update
              (Rendering|Material|SetScalarParameterValue "/Game/03_VFX/02_Material/00_Master/02_MPC/MPC_Slide.MPC_Slide" "Emissive" (Math|Float|Lerp 5e+01 0.0 _emissive) :!class /Script/Engine.KismetMaterialLibrary)
              (Rendering|Material|SetScalarParameterValue "/Game/03_VFX/02_Material/00_Master/02_MPC/MPC_Slide.MPC_Slide" "Desaturation" (Math|Float|Lerp 0.0 1.0 _desaturation) :!class /Script/Engine.KismetMaterialLibrary)
              (Rendering|Material|SetScalarParameterValue "/Game/03_VFX/02_Material/00_Master/02_MPC/MPC_Slide.MPC_Slide" "Fade" (Math|Float|Lerp 1.0 0.0 _fade) :!class /Script/Engine.KismetMaterialLibrary))
            (:Finished
              (Actor|DestroyActor))))
        (:else)))))

(fn ConstructionScript)