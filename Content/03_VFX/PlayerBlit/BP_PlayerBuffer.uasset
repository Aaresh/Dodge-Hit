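; Player buffer actor that tracks the player and four elephants in a render target covering a world-space square around its preview plane.
; Each tick it publishes player position to an MPC, reads elephant positions from it and converts all to UVs for the plane's material.
; A blit material is drawn into the render target, which feeds a world-projection plane along with the bounds.
; Cell size times pixel count sets the covered area.
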(event EventBeginPlay
  (bind _worldcellsize (Variables|Default|GetWorldCellSize))
  (bind _bufferpixelsize (Variables|Default|GetBufferPixelSize))
  (bind _previewplane (Variables|Default|GetPreviewPlane))
  (bind _bufferpixelsize_2 (Variables|Default|GetBufferPixelSize))
  (bind _worldprojectplane (Variables|Default|GetWorldProjectPlane))
  (bind _previewplane_2 (Variables|Default|GetPreviewPlane))
  (bind _returnvalue (Transformation|GetWorldLocation _previewplane_2))
  (bind _returnvalue_2 (* _worldcellsize _bufferpixelsize))
  (bind _staticmeshcomponent (Variables|/Script/Engine.StaticMeshActor|GetStaticMeshComponent _worldprojectplane))
  (bind _returnvalue_3 (* 0.5 _returnvalue_2))
  (bind _returnvalue_4 (Math|Vector|MakeVector _returnvalue_3 _returnvalue_3 0.0))
  (Variables|Default|SetMaxBounds (+ _returnvalue _returnvalue_4))
  (Variables|Default|SetMinBounds (- _returnvalue _returnvalue_4))
  (Transformation|SetWorldScale3D _previewplane (Math|Conversions|ToVector(Float) (/ _returnvalue_2 1e+02)))
  (bind _returnvalue_5 (Rendering|CreateRenderTarget2D _bufferpixelsize_2 _bufferpixelsize_2 "RTF_RGBA16f" "(R=0.000000,G=0.000000,B=0.000000,A=1.000000)" true true))
  (Variables|Default|SetRT_Final _returnvalue_5)
  (bind _returnvalue_6 (Rendering|Material|CreateDynamicMaterialInstance (Variables|Default|GetPreviewPlane) 0 "/Game/04_VFX/PlayerBlit/MT_PlayerBuffer_Blit.MT_PlayerBuffer_Blit" "None" :!class /Script/Engine.PrimitiveComponent))
  (bind _output_get (Variables|Default|SetMID_Blit _returnvalue_6))
  (Rendering|Material|SetTextureParameterValue _output_get "RenderTarget" (Variables|Default|GetRT_Final))
  (bind _returnvalue_7 (Rendering|Material|CreateDynamicMaterialInstance (Variables|Default|GetPreviewPlane) 0 (Rendering|Material|GetMaterial _previewplane 0) "None" :!class /Script/Engine.PrimitiveComponent))
  (bind _output_get_2 (Variables|Default|SetMID_Preview _returnvalue_7))
  (Rendering|Material|SetTextureParameterValue _output_get_2 "RenderTarget" (Variables|Default|GetRT_Final))
  (bind _returnvalue_8 (Rendering|Material|CreateDynamicMaterialInstance _staticmeshcomponent 0 (Rendering|Material|GetMaterial _staticmeshcomponent 0) "None" :!class /Script/Engine.PrimitiveComponent))
  (Variables|Default|SetMID_WorldPorjectPlane _returnvalue_8))

(event EventTick
  (params (DeltaSeconds :type Float%20%28single-precision%29))
  (bind _minbounds (Variables|Default|GetMinBounds))
  (bind _maxbounds (Variables|Default|GetMaxBounds))
  (|ElephantLocation01)
  (|ElephantLocation02)
  (|ElephantLocation03)
  (|ElephantLocation04)
  (|PlayerLocationUVSpace)
  (Rendering|Material|SetTextureParameterValue (Variables|Default|GetMID_Blit) "RenderTarget" 0)
  (Rendering|DrawMaterialtoRenderTarget (Variables|Default|GetRT_Final) (Variables|Default|GetMID_Blit))
  (Rendering|Material|SetVectorParameterValue (Variables|Default|GetMID_WorldPorjectPlane) "MinMaxBounds" (Utilities|Struct|MakeLinearColor (.x _minbounds) (.x _maxbounds) (.y _minbounds) (.y _maxbounds)) :!class /Script/Engine.MaterialInstanceDynamic)
  (Rendering|Material|SetTextureParameterValue (Variables|Default|GetMID_WorldPorjectPlane) "Buffer" (Variables|Default|GetRT_Final)))

(fn ConstructionScript
  (bind _worldcellsize (Variables|Default|GetWorldCellSize))
  (bind _bufferpixelsize (Variables|Default|GetBufferPixelSize))
  (bind _previewplane (Variables|Default|GetPreviewPlane))
  (bind _returnvalue (Transformation|GetWorldLocation _previewplane))
  (bind _returnvalue_2 (* _worldcellsize _bufferpixelsize))
  (bind _returnvalue_3 (* 0.5 _returnvalue_2))
  (bind _returnvalue_4 (Math|Vector|MakeVector _returnvalue_3 _returnvalue_3 0.0))
  (Variables|Default|SetMaxBounds (+ _returnvalue _returnvalue_4))
  (Variables|Default|SetMinBounds (- _returnvalue _returnvalue_4))
  (Transformation|SetWorldScale3D (Variables|Default|GetPreviewPlane) (Math|Conversions|ToVector(Float) (/ _returnvalue_2 1e+02))))