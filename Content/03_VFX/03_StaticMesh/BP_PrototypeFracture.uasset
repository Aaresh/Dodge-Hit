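; BP_PrototypeFracture is a short-lived destruction effect that shows a fractured mesh for one of two characters, chosen by IndexChara.
; On BeginPlay it reveals the matching GCPlayer component, tints the NSDestruction particles blue or red and activates them.
; After a brief delay it enables gravity on both GCPlayer components, spawns two randomly rotated splash decals, then destroys itself two seconds later.
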(event EventBeginPlay
  (bind _ns_destruction (Variables|Default|GetNS_Destruction))
  (bind _gc_player02 (Variables|Default|GetGC_Player02))
  (bind _gc_player01 (Variables|Default|GetGC_Player01))
  (if (== (Variables|Default|GetIndexChara) 0)
    (Development|SetHiddeninGame _gc_player01 false false)
    (Development|SetHiddeninGame _gc_player02 true false)
    (Niagara|SetNiagaraVariable(LinearColor) _ns_destruction "ParticleColor" (Variables|Default|GetBlueColor))
    (else
      (Development|SetHiddeninGame _gc_player01 true false)
      (Development|SetHiddeninGame _gc_player02 false false)
      (Niagara|SetNiagaraVariable(LinearColor) _ns_destruction "ParticleColor" (Variables|Default|GetRedColor))))
  (Components|Activation|Activate _ns_destruction false)
  (Utilities|FlowControl|Delay 0.1)
  (bind _output_get (Variables|Default|SetGravity%20Enabled true))
  (Physics|SetEnableGravity (Variables|Default|GetGC_Player02) _output_get)
  (Utilities|FlowControl|Sequence
    (:then_0
      (Utilities|FlowControl|Delay 2.0)
      (Actor|DestroyActor))
    (:then_1
      (Utilities|FlowControl|Delay 0.2)
      (Rendering|Decal|SpawnDecalatLocation "/Game/03_VFX/02_Material/Mi_SplashDecal.Mi_SplashDecal" "256.000000,150.000000,150.000000" (Transformation|GetActorLocation) (Math|Rotator|MakeRotator (Math|Random|RandomFloatinRange -1.8e+02 1.8e+02) -9e+01 (Math|Random|RandomFloatinRange -1.8e+02 1.8e+02)) 2.0)
      (Rendering|Decal|SpawnDecalatLocation "/Game/03_VFX/02_Material/Mi_SplashDecal.Mi_SplashDecal" "256.000000,150.000000,150.000000" (Transformation|GetActorLocation) (Math|Rotator|MakeRotator (Math|Random|RandomFloatinRange -1.8e+02 1.8e+02) -9e+01 (Math|Random|RandomFloatinRange -1.8e+02 1.8e+02)) 2.0))))

(fn ConstructionScript)