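; Player death effect actor that shows a character-specific destruction burst with a splash decal, then cleans itself up.
; On BeginPlay, IndexChara selects which player Geometry Collection is visible and tints the Niagara destruction particles blue or red.
; After a short delay, it spawns a random splash decal at its location and enables gravity on both collections.
; The actor destroys itself a few seconds later.
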(event EventBeginPlay
  (bind _ns_destruction (Variables|Default|GetNS_Destruction))
  (bind _gc_player02 (Variables|Default|GetGC_Player02))
  (bind _gc_player01 (Variables|Default|GetGC_Player01))
  (if (== (Variables|Default|GetIndexChara) 0)
    (Development|SetHiddeninGame _gc_player01 false false)
    (Development|SetHiddeninGame _gc_player02 true false)
    (Niagara|SetNiagaraVariable(LinearColor) _ns_destruction "ParticleColor" (Variables|Default|GetBlueColor))
    (else
      (Development|SetHiddeninGame _gc_player01 true false)
      (Development|SetHiddeninGame _gc_player02 false false)
      (Niagara|SetNiagaraVariable(LinearColor) _ns_destruction "ParticleColor" (Variables|Default|GetRedColor))))
  (Components|Activation|Activate _ns_destruction false)
  (Utilities|FlowControl|Delay 0.1)
  (Rendering|Decal|SpawnDecalatLocation (Utilities|Select :Index (Math|Random|RandomInteger 3) :Option%200 "/Game/03_VFX/02_Material/02_Enviro/Mi_SplashDecal.Mi_SplashDecal" :Option%201 "/Game/03_VFX/02_Material/02_Enviro/Mi_SplashDecal02.Mi_SplashDecal02" :Option%202 "/Game/03_VFX/02_Material/02_Enviro/Mi_SplashDecal03.Mi_SplashDecal03") "256.000000,256.000000,256.000000" (Transformation|GetActorLocation) "-90.000000,0.000000,0.000000" 3.0)
  (bind _output_get (Variables|Default|SetGravity%20Enabled true))
  (Physics|SetEnableGravity (Variables|Default|GetGC_Player02) _output_get)
  (Utilities|FlowControl|Delay 4.0)
  (Actor|DestroyActor))

(fn ConstructionScript)