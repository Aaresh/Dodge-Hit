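; Player 2 dash VFX actor that leaves a fading Quinn afterimage in a frozen pose.
; On BeginPlay it copies the pose from the supplied skeletal component onto its poseable mesh, if that component is valid.
; It assigns dynamic P2 VFX materials to both mesh slots, and a timeline drives their Fade parameter.
; The actor destroys itself after a short delay once the timeline finishes.
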(event EventBeginPlay
  (bind _poseablemesh (Variables|Default|GetPoseableMesh))
  (bind _in_component_to_copy (Variables|Default|GetIn%20Component%20to%20Copy)
    (:then
      (Class|PoseableMeshComponent|CopyPosefromSkeletalComponent (Variables|Default|GetPoseableMesh) _in_component_to_copy)
      (Utilities|FlowControl|Sequence
        (:then_0
          (bind _returnvalue (Rendering|Material|CreateDynamicMaterialInstance "/Game/X_BaseContent/02_Characters/Mannequins/Materials/Quinn/MI_Quinn2_P2_VFX.MI_Quinn2_P2_VFX" "FirstMat" "None" :!class /Script/Engine.KismetMaterialLibrary))
          (bind _output_get (Variables|Default|SetDM_FirstMat _returnvalue))
          (Rendering|Material|SetMaterial _poseablemesh 0 _output_get)
          (bind _newtrack_0 (Timeline|Timeline PlayFromStart)
            (:Update
              (Rendering|Material|SetScalarParameterValue (Variables|Default|GetDM_FirstMat) "Fade" _newtrack_0 :!class /Script/Engine.MaterialInstanceDynamic)
              (Rendering|Material|SetScalarParameterValue (Variables|Default|GetDM_SecondMat) "Fade" _newtrack_0 :!class /Script/Engine.MaterialInstanceDynamic))
            (:Finished
              (Utilities|FlowControl|Delay 1.0)
              (Actor|DestroyActor))))
        (:then_1
          (bind _returnvalue_2 (Rendering|Material|CreateDynamicMaterialInstance "/Game/X_BaseContent/02_Characters/Mannequins/Materials/Quinn/MI_Quinn1_P2_VFX.MI_Quinn1_P2_VFX" "SecondMat" "None" :!class /Script/Engine.KismetMaterialLibrary))
          (bind _output_get_2 (Variables|Default|SetDM_SecondMat _returnvalue_2))
          (Rendering|Material|SetMaterial _poseablemesh 1 _output_get_2)
          (Timeline|Timeline PlayFromStart))))
    (:else)))

(fn ConstructionScript)